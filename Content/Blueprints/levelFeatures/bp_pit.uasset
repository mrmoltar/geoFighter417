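; Pit level feature for a tile-based map that damages a player who falls into it and sends them back to their starting tile.
; On BeginPlay it marks its tile impassable, hides the tile mesh and registers itself as that tile's occupant.
; The fall event moves the player onto the hit tile, pauses briefly, returns them ignoring move range, applies pit damage and re-registers the pit on the hit tile.
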(event Custom|fallInPit
  (bind _playercontrollerref (Variables|Default|GetplayerControllerRef))
  (bind _playercontrollerref_2 (Variables|Default|GetplayerControllerRef))
  (bind _playerref (Variables|/Game/Blueprints/controllers/bp_ctlr_player.bp_ctlr_player_C|GetplayerRef _playercontrollerref_2))
  (Default|MovePlayertoActor _playercontrollerref (Variables|/Game/Blueprints/controllers/bp_ctlr_player.bp_ctlr_player_C|GethitTile _playercontrollerref) false)
  (Utilities|FlowControl|Delay 0.5)
  (Default|MovePlayertoActor (Variables|Default|GetplayerControllerRef) (Variables|/Game/Blueprints/bp_player.bp_player_C|GetstartingTile _playerref) true)
  (Default|TakeDamage _playerref (Variables|Default|GetpitDamage))
  (Variables|/Game/Blueprints/bp_gridSquare.bp_gridSquare_C|SetactorHere (Variables|/Game/Blueprints/controllers/bp_ctlr_player.bp_ctlr_player_C|GethitTile (Variables|Default|GetplayerControllerRef)) self))

(event EventBeginPlay
  (bind _currenttile (Variables|Default|GetcurrentTile))
  (Variables|/Game/Blueprints/bp_gridSquare.bp_gridSquare_C|Setimpassable? _currenttile true)
  (Rendering|SetVisibility (Variables|/Game/Blueprints/bp_gridSquare.bp_gridSquare_C|GetStaticMesh _currenttile) false false)
  (Variables|/Game/Blueprints/bp_gridSquare.bp_gridSquare_C|SetactorHere (Variables|Default|GetcurrentTile) self))

(fn ConstructionScript)
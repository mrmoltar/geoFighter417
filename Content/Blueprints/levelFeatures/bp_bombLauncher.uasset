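; Grid-based bomb launcher level feature that faces one of four compass directions and spawns bombs on tiles ahead of it.
; BeginPlay applies the facing, and Rotate steps it to the next direction and re-arms shooting.
; Shoot spawns a registered bomb on the passable, empty tile at the given distance, then disarms.
; An occupied tile triggers a recursive retry at BombDistance minus one, rather than decrementing the passed distance.
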(event EventBeginPlay
  (Transformation|SetActorRotation (Utilities|Select :Index (Variables|Default|Getdirection) :NewEnumerator0 "0,90.000000, 0" :NewEnumerator1 "0.000000,180.000000,0.000000" :NewEnumerator2 "0.000000,-90.000000,0.000000" :NewEnumerator3 "0, 0, 0" :NewEnumerator8 "0, 0, 0")))

(event Collision|EventActorBeginOverlap
  (params (OtherActor :type Actor%20Object%20Reference)))

(event EventTick
  (params (DeltaSeconds :type Float%20%28single-precision%29)))

(fn ConstructionScript)

(fn Rotate
  (Variables|Default|SetcanShoot? true)
  (bind _output_get (Variables|Default|Setdirection (Utilities|Select :Index (Variables|Default|Getdirection) :NewEnumerator0 "NewEnumerator1" :NewEnumerator1 "NewEnumerator2" :NewEnumerator2 "NewEnumerator3" :NewEnumerator3 "NewEnumerator0" :NewEnumerator8 "NewEnumerator8")))
  (Transformation|SetWorldRotation (Variables|Default|GetDefaultSceneRoot) (Utilities|Select :Index _output_get :NewEnumerator0 "0,90.000000, 0" :NewEnumerator1 "0.000000,180.000000,0.000000" :NewEnumerator2 "0.000000,-90.000000,0.000000" :NewEnumerator3 "0, 0, 0" :NewEnumerator8 "0, 0, 0") false false))

(fn Shoot
  (params (shootDistance :type Integer))
  (if (== shootDistance 0)
    (return)
    (elif (Variables|Default|GetcanShoot?)
      (bind _array_element (CallFunction|GetGridSquarefromCoords (Variables|/Game/Blueprints/controllers/bp_ctlr_player.bp_ctlr_player_C|GetgridArray (Variables|Default|GetplayerControllerRef)) (+ (* (Utilities|Select :Index (Variables|Default|Getdirection) :NewEnumerator0 "0,1.000000,0.000000" :NewEnumerator1 "-1.000000,0.000000,0.000000" :NewEnumerator2 "0.000000,-1.000000,0.000000" :NewEnumerator3 "1.000000,0.000000,0.000000" :NewEnumerator8 "0, 0, 0") shootDistance) (Variables|/Game/Blueprints/bp_gridSquare.bp_gridSquare_C|GetcurrentCoords (Variables|Default|GetcurrentTile)))))
      (Utilities|IsValid (Variables|/Game/Blueprints/bp_gridSquare.bp_gridSquare_C|GetactorHere _array_element)
        (:Is%20Valid
          (CallFunction|Shoot (- (Variables|Default|GetbombDistance) 1))
          (return))
        (:Is%20Not%20Valid
          (if (not (Variables|/Game/Blueprints/bp_gridSquare.bp_gridSquare_C|Getimpassable? _array_element))
            (bind _returnvalue (Game|SpawnActorfromClass "/Game/Blueprints/levelFeatures/bp_bomb.bp_bomb_C" (Math|Transform|MakeTransform (Math|Vector|MakeVector (.x (Transformation|GetWorldLocation (Variables|/Game/Blueprints/bp_gridSquare.bp_gridSquare_C|GetStaticMesh _array_element))) (.y (Transformation|GetWorldLocation (Variables|/Game/Blueprints/bp_gridSquare.bp_gridSquare_C|GetStaticMesh _array_element))) 2e+01) "0, 0, 0" "1,1,1") "Undefined" 0 _array_element (Variables|Default|GetrhythmControllerRef) 0))
            (Utilities|Array|Add (Variables|/Game/Blueprints/controllers/bp_ctlr_levelFeatures.bp_ctlr_levelFeatures_C|GetbombRefs (Variables|/Game/Blueprints/controllers/bp_ctlr_player.bp_ctlr_player_C|GetlevelFeatureControllerRef (Variables|Default|GetplayerControllerRef))) _returnvalue)
            (Variables|Default|SetcanShoot? false)
            (return)))))))
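; Floor spike trap feature for a tile-based level that damages whoever stands on it and blocks the tile while raised.
; ExtendSpikes shows the spike mesh, marks the current tile impassable, and applies spike damage to a player or enemy occupying it.
; RetractSpikes hides the mesh and makes the tile passable again.
; The event graph is empty, so both functions rely on external callers.
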(event EventBeginPlay)

(event Collision|EventActorBeginOverlap
  (params (OtherActor :type Actor%20Object%20Reference)))

(event EventTick
  (params (DeltaSeconds :type Float%20%28single-precision%29)))

(fn ConstructionScript)

(fn ExtendSpikes
  (bind _currenttile (Variables|Default|GetcurrentTile))
  (bind _actorhere (Variables|/Game/Blueprints/bp_gridSquare.bp_gridSquare_C|GetactorHere _currenttile))
  (Rendering|SetVisibility (Variables|Default|Getspikes_mesh) true false)
  (Variables|Default|SetspikesExtended? true)
  (Utilities|IsValid _currenttile
    (:Is%20Valid
      (Variables|/Game/Blueprints/bp_gridSquare.bp_gridSquare_C|Setimpassable? _currenttile true)
      (bind _asbp_player (Utilities|Casting|CastTobp_player _actorhere)
        (:then
          (Default|TakeDamage _asbp_player (Variables|Default|GetspikeDamage)))
        (:CastFailed
          (bind _asbp_enemy_parent (Utilities|Casting|CastTobp_enemy_parent _actorhere))
          (Default|TakeDamage _asbp_enemy_parent (Variables|Default|GetspikeDamage)))))))

(fn RetractSpikes
  (bind _currenttile (Variables|Default|GetcurrentTile))
  (Rendering|SetVisibility (Variables|Default|Getspikes_mesh) false false)
  (Variables|Default|SetspikesExtended? false)
  (Utilities|IsValid _currenttile
    (:Is%20Valid
      (Variables|/Game/Blueprints/bp_gridSquare.bp_gridSquare_C|Setimpassable? _currenttile false))))
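; Room square Blueprint for a grid level layout, displaying its door directions, H value and coordinates.
; Its updateArrows event shows the N, E, S or W arrow for each DoorArray entry and hides all four only when the array is empty.
; The same loop removes one other enumerator value from the array while iterating it.
; The event then writes HValue and the floored X.Y coordinates to text components.
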(event Custom|updateArrows
  (bind _coords (Variables|Default|Getcoords))
  (bind _doorarray (Variables|Default|GetdoorArray))
  (Utilities|FlowControl|Sequence
    (:then_0
      (if (> (Utilities|Array|Length _doorarray) 0)
        (for _array_element _doorarray
          (if (Utilities|Enum|Equal(Enum) _array_element "NewEnumerator0")
            (Rendering|SetVisibility (Variables|Default|GetNArrow) true false)
            (elif (Utilities|Enum|Equal(Enum) _array_element "NewEnumerator1")
              (Rendering|SetVisibility (Variables|Default|GetEArrow) true false)
              (elif (Utilities|Enum|Equal(Enum) _array_element "NewEnumerator2")
                (Rendering|SetVisibility (Variables|Default|GetSArrow) true false)
                (elif (Utilities|Enum|Equal(Enum) _array_element "NewEnumerator3")
                  (Rendering|SetVisibility (Variables|Default|GetWArrow) true false)
                  (elif (Utilities|Enum|Equal(Enum) _array_element "NewEnumerator8")
                    (Utilities|Array|RemoveItem (Variables|Default|GetdoorArray) _array_element)))))))
        (else
          (Rendering|SetVisibility (Variables|Default|GetNArrow) false false)
          (Rendering|SetVisibility (Variables|Default|GetEArrow) false false)
          (Rendering|SetVisibility (Variables|Default|GetSArrow) false false)
          (Rendering|SetVisibility (Variables|Default|GetWArrow) false false))))
    (:then_1
      (Rendering|Components|TextRender|SetText (Variables|Default|GethValueText) (Utilities|Text|ToText(String) (Utilities|String|ToString(Integer) (Variables|Default|Get%20hValue))))
      (Rendering|Components|TextRender|SetText (Variables|Default|GetcoordText) (Utilities|Text|ToText(String) (Utilities|String|Append (Utilities|String|ToString(Integer) (Math|Float|Floor (.x _coords))) "." (Utilities|String|ToString(Integer) (Math|Float|Floor (.y _coords)))))))))

(event EventBeginPlay)

(event Collision|EventActorBeginOverlap
  (params (OtherActor :type Actor%20Object%20Reference)))

(event EventTick
  (params (DeltaSeconds :type Float%20%28single-precision%29)))

(fn ConstructionScript)
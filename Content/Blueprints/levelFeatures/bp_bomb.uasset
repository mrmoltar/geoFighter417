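; Grid-based bomb level feature that blocks its tile and damages players on nearby tiles when it explodes.
; On explode it hides its sphere, plays a clap sound, damages any player on tiles gathered within radius one, then frees its tile.
; Neighbour lookup scans a square of the player controller's flattened grid array, reached through the rhythm controller.
; TimerAndExplode only removes the bomb from the level feature controller's list.
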(event Custom|explode
  (bind _currenttile (Variables|Default|GetcurrentTile))
  (bind _currentcoords (Variables|/Game/Blueprints/bp_gridSquare.bp_gridSquare_C|GetcurrentCoords _currenttile))
  (Rendering|SetVisibility (Variables|Default|GetSphere) false true)
  (Audio|PlaySound2D "/Game/sounds/DNC_Clap_6.DNC_Clap_6")
  (bind _surroundingtiles1 (CallFunction|GetSurroundingTiles 1 (Math|Float|Truncate (.x _currentcoords)) (Math|Float|Truncate (.y _currentcoords))))
  (for _array_element _surroundingtiles1
    (bind _asbp_player (Utilities|Casting|CastTobp_player (Variables|/Game/Blueprints/bp_gridSquare.bp_gridSquare_C|GetactorHere _array_element)))
    (Default|TakeDamage _asbp_player (Variables|Default|Getdamage)))
  (Variables|/Game/Blueprints/bp_gridSquare.bp_gridSquare_C|Setimpassable? (Variables|Default|GetcurrentTile) false)
  (Variables|/Game/Blueprints/bp_gridSquare.bp_gridSquare_C|SetactorHere (Variables|Default|GetcurrentTile) 0))

(event EventBeginPlay
  (Variables|/Game/Blueprints/bp_gridSquare.bp_gridSquare_C|Setimpassable? (Variables|Default|GetcurrentTile) true))

(event Collision|EventActorBeginOverlap
  (params (OtherActor :type Actor%20Object%20Reference)))

(fn ConstructionScript)

(fn GetSurroundingTiles
  (params (radius :type Integer) (currentX :type Integer) (currentY :type Integer))
  (bind _rhythmcontroller (Variables|Default|GetrhythmController))
  (bind _rhythmcontroller_2 (Variables|Default|GetrhythmController))
  (bind _playerctlrref (Variables|/Game/Blueprints/controllers/bp_ctlr_rhythm.bp_ctlr_rhythm_C|GetplayerCtlrRef _rhythmcontroller_2))
  (bind _playerctlrref_2 (Variables|/Game/Blueprints/controllers/bp_ctlr_rhythm.bp_ctlr_rhythm_C|GetplayerCtlrRef _rhythmcontroller))
  (bind _output_get (LocalVariables|SetR radius))
  (LocalVariables|SetX (- currentX _output_get))
  (LocalVariables|SetY (- currentY _output_get))
  (for _index (range 0 radius)
    (LocalVariables|Seti (LocalVariables|Geti)))
  (LocalVariables|SetlocalArea (* (LocalVariables|Geti) (LocalVariables|Geti)))
  (for _index_2 (range 0 (- (LocalVariables|Geti) 1))
    (bind _element (Utilities|Get2dArray (Variables|/Game/Blueprints/controllers/bp_ctlr_player.bp_ctlr_player_C|GetgridArray _playerctlrref_2) (LocalVariables|GetX) (+ (LocalVariables|GetY) _index_2) (Variables|/Game/Blueprints/controllers/bp_ctlr_player.bp_ctlr_player_C|GetgridHorizontal _playerctlrref_2))
      (:1
        (Utilities|IsValid _element
          (:Is%20Valid
            (Utilities|Array|Add (LocalVariables|GetsurroundingTiles) _element))
          (:Is%20Not%20Valid
            _))
        (for _index_3 (range 1 (- (LocalVariables|Geti) 1))
          (bind _element_2 (Utilities|Get2dArray (Variables|/Game/Blueprints/controllers/bp_ctlr_player.bp_ctlr_player_C|GetgridArray _playerctlrref) (+ (LocalVariables|GetX) _index_3) (+ (LocalVariables|GetY) _index_2) (Variables|/Game/Blueprints/controllers/bp_ctlr_player.bp_ctlr_player_C|GetgridHorizontal _playerctlrref))
            (:1
              (Utilities|IsValid _element_2
                (:Is%20Valid
                  (Utilities|Array|Add (LocalVariables|GetsurroundingTiles) _element_2)))))))))
  (return (LocalVariables|GetsurroundingTiles)))

(fn TimerandExplode
  (Utilities|Array|RemoveItem (Variables|/Game/Blueprints/controllers/bp_ctlr_levelFeatures.bp_ctlr_levelFeatures_C|GetbombRefs (Variables|/Game/Blueprints/controllers/bp_ctlr_player.bp_ctlr_player_C|GetlevelFeatureControllerRef (Variables|/Game/Blueprints/controllers/bp_ctlr_rhythm.bp_ctlr_rhythm_C|GetplayerCtlrRef (Variables|Default|GetrhythmController)))) self))
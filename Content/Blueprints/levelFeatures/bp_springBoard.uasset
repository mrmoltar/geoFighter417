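; Spring board level feature that targets the neighboring grid tile in one of eight directions, shown by an arrow rotated at construction.
; On BeginPlay it finds that tile by searching the player controller's grid array for matching coordinates.
; SpringPlayer moves a player on its current tile to the target and plays a sound, though nothing here calls it.
; Tick only re-arms the Active flag from the rhythm controller's beat value.
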(event Custom|getTargetTile
  (bind _array_element (CallFunction|GetTilefromCoords (+ (Variables|/Game/Blueprints/bp_gridSquare.bp_gridSquare_C|GetcurrentCoords (Variables|Default|GetcurrentTile)) (Utilities|Select :Index (Variables|Default|GetmovementDir) :NewEnumerator0 "0,1.000000,0.000000" :NewEnumerator1 "-1.000000,0.000000,0.000000" :NewEnumerator2 "0.000000,-1.000000,0.000000" :NewEnumerator3 "1.000000,0.000000,0.000000" :NewEnumerator4 "-1.000000,1.000000,0.000000" :NewEnumerator5 "-1.000000,-1.000000,0.000000" :NewEnumerator6 "1.000000,-1.000000, 0" :NewEnumerator7 "1.000000,1.000000, 0" :NewEnumerator8 "0, 0, 0"))))
  (Variables|Default|SettargetTile _array_element))

(event EventBeginPlay
  (CallFunction|GetTargetTile))

(event Collision|EventActorBeginOverlap
  (params (OtherActor :type Actor%20Object%20Reference)))

(event EventTick
  (params (DeltaSeconds :type Float%20%28single-precision%29))
  (if (not (and (Variables|Default|Getactive?) (Math|Float|NearlyEqual(Float) (Variables|Default|GetbeatTrigger) (Variables|/Game/Blueprints/controllers/bp_ctlr_rhythm.bp_ctlr_rhythm_C|GetrhythmValue (Variables|Default|GetrhythmControllerRef)) 0.1)))
    (if (Math|Float|NearlyEqual(Float) 1.0 (Variables|/Game/Blueprints/controllers/bp_ctlr_rhythm.bp_ctlr_rhythm_C|GetrhythmValue (Variables|Default|GetrhythmControllerRef)) 0.1)
      (Variables|Default|Setactive? true))))

(fn ConstructionScript
  (Transformation|SetRelativeRotation (Variables|Default|GetArrow) (Math|Rotator|MakeRotator 0.0 0.0 (Utilities|Select :Index (Variables|Default|GetmovementDir) :NewEnumerator0 9e+01 :NewEnumerator1 1.8e+02 :NewEnumerator2 -9e+01 :NewEnumerator3 0.0 :NewEnumerator4 135.0 :NewEnumerator5 -135.0 :NewEnumerator6 -45.0 :NewEnumerator7 45.0 :NewEnumerator8 0.0)) false false))

(fn GetTilefromCoords
  (params (Coords :type Vector))
  (for _array_element (Variables|/Game/Blueprints/controllers/bp_ctlr_player.bp_ctlr_player_C|GetgridArray (Variables|Default|GetplayerControllerRef))
    (if (Math|Vector|Equal(Vector) (Variables|/Game/Blueprints/bp_gridSquare.bp_gridSquare_C|GetcurrentCoords _array_element) Coords 0.0001)
      (return _array_element))))

(fn SpringPlayer
  (Utilities|Casting|CastTobp_player (Variables|/Game/Blueprints/bp_gridSquare.bp_gridSquare_C|GetactorHere (Variables|Default|GetcurrentTile)))
  (Default|MovetoActor (Variables|Default|GetplayerControllerRef) (Variables|Default|GettargetTile) false)
  (Audio|PlaySound2D "/Game/sounds/reverseHit.reverseHit" 0.8 0.1))
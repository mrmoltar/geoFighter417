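; Level controller that procedurally generates a square grid room layout with a start and exit on opposite edges.
; BeginPlay spawns bp_roomSquare tiles scored by Manhattan distance to the exit.
; The a*Path event, actually a greedy walker with random tie-breaks, carves a doored path, then randomly branches extra rooms toward a target count.
; It finally copies tiles into RoomArray, destroys them and passes the array to bp_ctlr_player.
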(event Custom|a*Path
  (bind _levelsize (Variables|Default|GetlevelSize))
  (bind _levelsize_2 (Variables|Default|GetlevelSize))
  ;[1 1 1] a (star?) pathfinding
  (Utilities|FlowControl|Sequence
    (:then_0
      (Utilities|FlowControl|ForLoopwithBreak 0 (- (* _levelsize_2 _levelsize_2) 1) :!label _label
        (:LoopBody
          (bind _exit_ (CallFunction|PathtoExit))
          (if _exit_
            (for _array_element (Variables|Default|GetclosedList)
              (CallFunction|CreateDoors _array_element (Variables|/Game/Blueprints/bp_roomSquare.bp_roomSquare_C|GetparentTile _array_element))
              (CallFunction|CreateDoors _array_element (Variables|/Game/Blueprints/bp_roomSquare.bp_roomSquare_C|GetchildTile _array_element))
              (goto _label Break))))
        (:Completed
          (CallFunction|RemoveStartandEndfromClosedList))))
    (:then_1
      ;[1 1 1] add additional rooms
      (Utilities|FlowControl|ForLoopwithBreak 0 (- (* _levelsize _levelsize) 1) :!label _label_2
        (:LoopBody
          (bind _n1 (CallFunction|GetRoomNumber))
          (if (< _n1 (Variables|Default|GetdesiredRoomNumber))
            (CallFunction|RemoveStartandEndfromClosedList)
            (CallFunction|AddExtraRooms)
            (else
              (goto _label_2 Break))))
        (:Completed
          (CallFunction|UpdateStart&End))))
    (:then_2
      (CallFunction|UpdateTiles))
    (:then_3
      (Utilities|Array|Clear (Variables|Default|GetroomArray))
      ;[1 1 1] loop thru all tiles and apply all vars to roomStructArray
      (for _array_element_2 (Variables|Default|GetroomTileArray)
        (Utilities|Array|Add (Variables|Default|GetroomArray) (Utilities|Struct|Makestruct_room (Variables|/Game/Blueprints/bp_roomSquare.bp_roomSquare_C|GetdoorArray _array_element_2) (Variables|/Game/Blueprints/bp_roomSquare.bp_roomSquare_C|Getcoords _array_element_2) (Variables|/Game/Blueprints/bp_roomSquare.bp_roomSquare_C|GetstartHere? _array_element_2) (Variables|/Game/Blueprints/bp_roomSquare.bp_roomSquare_C|GetexitHere? _array_element_2) (Variables|/Game/Blueprints/bp_roomSquare.bp_roomSquare_C|Get%20hValue _array_element_2) "0, 0, 0" "0, 0, 0")))
      (CallFunction|DestroyRoomTileActors))))

(event EventBeginPlay
  (bind _levelsize (Variables|Default|GetlevelSize))
  (bind _levelsize_2 (Variables|Default|GetlevelSize))
  (bind _levelsize_3 (Variables|Default|GetlevelSize))
  (bind _levelsize_4 (Variables|Default|GetlevelSize))
  (bind _os (Variables|Default|Getos))
  (bind _levelsize_5 (Variables|Default|GetlevelSize))
  (Utilities|FlowControl|Sequence
    (:then_0
      ;[1 1 1] create room grid
      ;;[1 1 1] loop thru rooms and set coords
      (for _index (range 0 (- (* _levelsize_2 _levelsize_2) 1))
        (Utilities|Array|Add (Variables|Default|GetroomArray) (Utilities|Struct|Makestruct_room (Variables|Default|GetdefaultDoors) (Math|Vector|MakeVector (Math|Conversions|ToFloat(Integer) (Math|Integer|%(Integer) _index _levelsize)) (Math|Conversions|ToFloat(Integer) (/ _index _levelsize)) 0.0) false false 999 "0, 0, 0" "0, 0, 0"))
        (bind _returnvalue (Game|SpawnActorfromClass "/Game/Blueprints/bp_roomSquare.bp_roomSquare_C" (Math|Transform|MakeTransform (Math|Vector|MakeVector (* (Math|Integer|%(Integer) _index _levelsize) _os) (* (/ _index _levelsize) _os) 0.0) "0, 0, 0" "1,1,1") "Undefined" 0 false false (Math|Vector|MakeVector (Math|Conversions|ToFloat(Integer) (Math|Integer|%(Integer) _index _levelsize)) (Math|Conversions|ToFloat(Integer) (/ _index _levelsize)) 0.0) 0))
        (Utilities|Array|Add (Variables|Default|GetroomTileArray) _returnvalue))
      ;;[1 1 1] create start and exit
      (bind (_starttile _exittile) (CallFunction|SetStartVars (Math|Random|RandomIntegerinRange 0 (- (Variables|Default|GetlevelSize) 1)) (Math|Random|RandomIntegerinRange (- (* _levelsize_3 _levelsize_3) _levelsize_3) (- (* _levelsize_5 _levelsize_5) 1))))
      (Variables|Default|SetstartTile _starttile)
      (Variables|Default|SetexitTile _exittile)
      (Variables|Default|SetdesiredRoomNumber (- (* _levelsize_4 _levelsize_4) (+ _levelsize_4 _levelsize_4))))
    (:then_1
      ;[1 1 1] set heurestic val and update tile textures
      (for _array_element (Variables|Default|GetroomTileArray)
        (Variables|/Game/Blueprints/bp_roomSquare.bp_roomSquare_C|Set%20hValue _array_element (Math|Float|Truncate (+ (Math|Float|Absolute(Float) (.x (- (Variables|Default|GetexitCoords) (Variables|/Game/Blueprints/bp_roomSquare.bp_roomSquare_C|Getcoords _array_element)))) (Math|Float|Absolute(Float) (.y (- (Variables|Default|GetexitCoords) (Variables|/Game/Blueprints/bp_roomSquare.bp_roomSquare_C|Getcoords _array_element)))))))
        (Default|UpdateArrows _array_element)))
    (:then_2
      ;[1 1 1] add starting tile to closed list & set H value to 0
      (Variables|Default|SetwalkerCurrentCoords (Variables|Default|GetstartCoords))
      (bind _tile (CallFunction|GetTilefromCoords (Variables|Default|GetstartCoords)))
      (Utilities|Array|Add (Variables|Default|GetclosedList) _tile)
      (Variables|/Game/Blueprints/bp_roomSquare.bp_roomSquare_C|Set%20hValue _tile 0))))

(event Collision|EventActorBeginOverlap
  (params (OtherActor :type Actor%20Object%20Reference)))

(fn ConstructionScript)

(fn SetStartVars
  (params (randStart :type Integer) (randExit :type Integer))
  (bind _roomtilearray (Variables|Default|GetroomTileArray))
  (bind _roomtilearray_2 (Variables|Default|GetroomTileArray))
  (bind _roomarray (Variables|Default|GetroomArray))
  (bind _output (Utilities|Array|Get(acopy) _roomtilearray randExit))
  (bind _output_2 (Utilities|Array|Get(acopy) _roomtilearray_2 randStart))
  (bind _output_3 (Utilities|Array|Get(acopy) _roomarray randStart))
  (Variables|Default|SetstartCoords (.coords _output_3))
  (Variables|Default|SetwalkerCurrentCoords (.coords _output_3))
  (Variables|Default|SetwalkerPreviousCoords (.coords _output_3))
  (Variables|/Game/Blueprints/bp_roomSquare.bp_roomSquare_C|SetstartHere? _output_2 true)
  (Rendering|Material|SetMaterial (Variables|/Game/Blueprints/bp_roomSquare.bp_roomSquare_C|GetStaticMesh _output_2) 0 "/Engine/MapTemplates/Materials/BasicAsset03.BasicAsset03")
  (Variables|Default|SetexitCoords (.coords (Utilities|Array|Get(acopy) (Variables|Default|GetroomArray) randExit)))
  (Variables|/Game/Blueprints/bp_roomSquare.bp_roomSquare_C|SetexitHere? _output true)
  (Rendering|Material|SetMaterial (Variables|/Game/Blueprints/bp_roomSquare.bp_roomSquare_C|GetStaticMesh _output) 0 "/Engine/MapTemplates/Materials/BasicAsset01.BasicAsset01")
  (return _output_2 _output))

(fn GetTilefromCoords
  (params (coords :type Vector))
  (for _array_element (Variables|Default|GetroomTileArray)
    (if (Math|Vector|Equal(Vector) (Variables|/Game/Blueprints/bp_roomSquare.bp_roomSquare_C|Getcoords _array_element) coords 0.0001)
      (return _array_element))))

(fn UpdateStart&End
  (Rendering|Material|SetMaterial (Variables|/Game/Blueprints/bp_roomSquare.bp_roomSquare_C|GetStaticMesh (Variables|Default|GetstartTile)) 0 "/Engine/MapTemplates/Materials/BasicAsset03.BasicAsset03")
  (Rendering|Material|SetMaterial (Variables|/Game/Blueprints/bp_roomSquare.bp_roomSquare_C|GetStaticMesh (Variables|Default|GetexitTile)) 0 "/Engine/MapTemplates/Materials/BasicAsset01.BasicAsset01")
  (return (Math|Vector|Equal(Vector) (Variables|Default|GetwalkerCurrentCoords) (Variables|Default|GetexitCoords) 0.0001)))

(fn GetAdjacentTiles
  (params (coords :type Vector))
  (bind _levelsize (Variables|Default|GetlevelSize))
  (bind _equalhvaluetiles (LocalVariables|GetequalHValueTiles))
  (bind _equalhvaluetiles_2 (LocalVariables|GetequalHValueTiles))
  (bind _returnvalue (Utilities|Array|Length _equalhvaluetiles))
  (bind _returnvalue_2 (Math|Conversions|ToFloat(Integer) _levelsize))
  ;[1 1 1] calc if each direction is in the room grid
  (for _index (range 0 3)
    ;[1 1 1] check if start or exit is new tile. if not add to surrounding tile array
    (if (Math|Boolean|ANDBoolean (>= (.X (Math|Vector|BreakVector (+ coords (Utilities|Select :Index (Utilities|Select :Index _index :Option%200 "NewEnumerator0" :Option%201 "NewEnumerator1" :Option%202 "NewEnumerator2" :Option%203 "NewEnumerator3") :NewEnumerator0 "0.000000,1.000000,0.000000" :NewEnumerator1 "-1.000000,0.000000,0.000000" :NewEnumerator2 "0.000000,-1.000000,0.000000" :NewEnumerator3 "1.000000,0.000000, 0" :NewEnumerator8 "9999.000000, 0, 0")))) 0.0) (< (.X (Math|Vector|BreakVector (+ coords (Utilities|Select :Index (Utilities|Select :Index _index :Option%200 "NewEnumerator0" :Option%201 "NewEnumerator1" :Option%202 "NewEnumerator2" :Option%203 "NewEnumerator3") :NewEnumerator0 "0.000000,1.000000,0.000000" :NewEnumerator1 "-1.000000,0.000000,0.000000" :NewEnumerator2 "0.000000,-1.000000,0.000000" :NewEnumerator3 "1.000000,0.000000, 0" :NewEnumerator8 "9999.000000, 0, 0")))) _returnvalue_2) (>= (.Y (Math|Vector|BreakVector (+ coords (Utilities|Select :Index (Utilities|Select :Index _index :Option%200 "NewEnumerator0" :Option%201 "NewEnumerator1" :Option%202 "NewEnumerator2" :Option%203 "NewEnumerator3") :NewEnumerator0 "0.000000,1.000000,0.000000" :NewEnumerator1 "-1.000000,0.000000,0.000000" :NewEnumerator2 "0.000000,-1.000000,0.000000" :NewEnumerator3 "1.000000,0.000000, 0" :NewEnumerator8 "9999.000000, 0, 0")))) 0.0) (< (.Y (Math|Vector|BreakVector (+ coords (Utilities|Select :Index (Utilities|Select :Index _index :Option%200 "NewEnumerator0" :Option%201 "NewEnumerator1" :Option%202 "NewEnumerator2" :Option%203 "NewEnumerator3") :NewEnumerator0 "0.000000,1.000000,0.000000" :NewEnumerator1 "-1.000000,0.000000,0.000000" :NewEnumerator2 "0.000000,-1.000000,0.000000" :NewEnumerator3 "1.000000,0.000000, 0" :NewEnumerator8 "9999.000000, 0, 0")))) _returnvalue_2))
      (bind _tile (CallFunction|GetTilefromCoords (+ coords (Utilities|Select :Index (Utilities|Select :Index _index :Option%200 "NewEnumerator0" :Option%201 "NewEnumerator1" :Option%202 "NewEnumerator2" :Option%203 "NewEnumerator3") :NewEnumerator0 "0.000000,1.000000,0.000000" :NewEnumerator1 "-1.000000,0.000000,0.000000" :NewEnumerator2 "0.000000,-1.000000,0.000000" :NewEnumerator3 "1.000000,0.000000, 0" :NewEnumerator8 "9999.000000, 0, 0"))))
      (if (Variables|/Game/Blueprints/bp_roomSquare.bp_roomSquare_C|GetexitHere? _tile)
        (LocalVariables|SetexitHere? (Variables|/Game/Blueprints/bp_roomSquare.bp_roomSquare_C|GetexitHere? _tile))
        (elif (not (Variables|/Game/Blueprints/bp_roomSquare.bp_roomSquare_C|GetstartHere? _tile))
          (Utilities|Array|Add (LocalVariables|GetsurroundingTiles) _tile)))))
  (for _array_element (LocalVariables|GetsurroundingTiles)
    (if (< (Variables|/Game/Blueprints/bp_roomSquare.bp_roomSquare_C|Get%20hValue _array_element) (LocalVariables|GetlowestHValue))
      (LocalVariables|SetlowestHValue (Variables|/Game/Blueprints/bp_roomSquare.bp_roomSquare_C|Get%20hValue _array_element))
      (bind _output_get (LocalVariables|SetlowestHValueTile _array_element))
      (Utilities|Array|Clear _equalhvaluetiles_2)
      (Utilities|Array|Add _equalhvaluetiles_2 _output_get)
      (elif (== (Variables|/Game/Blueprints/bp_roomSquare.bp_roomSquare_C|Get%20hValue _array_element) (LocalVariables|GetlowestHValue))
        (Utilities|Array|Add (LocalVariables|GetequalHValueTiles) _array_element))))
  (if (> _returnvalue 1)
    (return (Utilities|Array|Get(acopy) (LocalVariables|GetequalHValueTiles) (Math|Random|RandomIntegerinRange 0 (- _returnvalue 1))) (LocalVariables|GetexitHere?) (LocalVariables|GetsurroundingTiles))
    (else
      (return (LocalVariables|GetlowestHValueTile) (LocalVariables|GetexitHere?) (LocalVariables|GetsurroundingTiles)))))

(fn CreateDoors
  (params (startTile :type Bp%20Room%20Square%20Object%20Reference) (tileToCheck :type Bp%20Room%20Square%20Object%20Reference))
  (bind _coords (Variables|/Game/Blueprints/bp_roomSquare.bp_roomSquare_C|Getcoords tileToCheck))
  (bind _coords_2 (Variables|/Game/Blueprints/bp_roomSquare.bp_roomSquare_C|Getcoords startTile))
  (bind _doorarray (Variables|/Game/Blueprints/bp_roomSquare.bp_roomSquare_C|GetdoorArray startTile))
  (bind _returnvalue (- _coords _coords_2))
  (bind (_x _y) (Math|Vector|BreakVector _returnvalue))
  (if (and (Utilities|IsValid startTile) (Utilities|IsValid tileToCheck))
    (if (== _x 1.0)
      (if (== (Utilities|Array|FindItem _doorarray "NewEnumerator3") -1)
        (Utilities|Array|Add _doorarray "NewEnumerator3")
        (else
          (if (== _x -1.0) :!label _label
            (if (== (Utilities|Array|FindItem _doorarray "NewEnumerator1") -1)
              (Utilities|Array|Add _doorarray "NewEnumerator1")
              (else
                (if (== _y 1.0) :!label _label_2
                  (if (== (Utilities|Array|FindItem _doorarray "NewEnumerator0") -1)
                    (Utilities|Array|Add _doorarray "NewEnumerator0")
                    (else
                      (if (== _y -1.0) :!label _label_3
                        (if (== (Utilities|Array|FindItem _doorarray "NewEnumerator2") -1)
                          (Utilities|Array|Add _doorarray "NewEnumerator2")
                          (else
                            (return)))
                        (else
                          (return)))))
                  (else
                    (goto _label_3)))))
            (else
              (goto _label_2)))))
      (else
        (goto _label)))
    (return)
    (else
      (return))))

(fn PathtoExit
  (bind _tile (CallFunction|GetTilefromCoords (Variables|Default|GetwalkerCurrentCoords)))
  (LocalVariables|SetwalkerTile _tile)
  (bind (_lowesthvaluetile1 _atexit_) (CallFunction|GetAdjacentTiles (Variables|Default|GetwalkerCurrentCoords)))
  (LocalVariables|SetatExit? _atexit_)
  (LocalVariables|SetlowestHTile _lowesthvaluetile1)
  (if (LocalVariables|GetatExit?)
    (Variables|/Game/Blueprints/bp_roomSquare.bp_roomSquare_C|SetparentTile (Variables|Default|GetexitTile) (LocalVariables|GetwalkerTile))
    (Variables|/Game/Blueprints/bp_roomSquare.bp_roomSquare_C|SetchildTile (LocalVariables|GetwalkerTile) (Variables|Default|GetexitTile))
    (Utilities|Array|Add (Variables|Default|GetclosedList) (Variables|Default|GetexitTile))
    (return true)
    (else
      (Utilities|Array|Add (Variables|Default|GetclosedList) (LocalVariables|GetlowestHTile))
      (Variables|/Game/Blueprints/bp_roomSquare.bp_roomSquare_C|SetchildTile (LocalVariables|GetwalkerTile) (LocalVariables|GetlowestHTile))
      (Variables|/Game/Blueprints/bp_roomSquare.bp_roomSquare_C|SetparentTile (LocalVariables|GetlowestHTile) (LocalVariables|GetwalkerTile))
      (Variables|Default|SetwalkerCurrentCoords (Variables|/Game/Blueprints/bp_roomSquare.bp_roomSquare_C|Getcoords (LocalVariables|GetlowestHTile)))
      (Rendering|Material|SetMaterial (Variables|/Game/Blueprints/bp_roomSquare.bp_roomSquare_C|GetStaticMesh (LocalVariables|GetlowestHTile)) 0 "/Game/materials/m_tileBasic4.m_tileBasic4")
      (return false))))

(fn AddExtraRooms
  (bind _levelsize (Variables|Default|GetlevelSize))
  (bind _adjacenttiles (LocalVariables|GetadjacentTiles))
  (bind _closedlist (Variables|Default|GetclosedList))
  (bind _returnvalue (Utilities|Array|Length _closedlist))
  (bind _returnvalue_2 (Utilities|Array|Length _adjacenttiles))
  (bind _returnvalue_3 (Math|Conversions|ToFloat(Integer) _levelsize))
  (bind _returnvalue_4 (- _returnvalue 1))
  (bind _returnvalue_5 (- _returnvalue_2 1))
  (bind _returnvalue_6 (Math|Random|RandomIntegerinRange 0 _returnvalue_4))
  (bind _returnvalue_7 (Math|Random|RandomIntegerinRange 0 _returnvalue_5))
  (bind _output (Utilities|Array|Get(acopy) _closedlist _returnvalue_6))
  (bind _output_2 (Utilities|Array|Get(acopy) _adjacenttiles _returnvalue_7))
  (Utilities|IsValid _output
    (:Is%20Valid
      (LocalVariables|SetchosenTile _output)
      (for _index (range 0 3)
        (if (Math|Boolean|ANDBoolean (>= (.X (Math|Vector|BreakVector (+ (Variables|/Game/Blueprints/bp_roomSquare.bp_roomSquare_C|Getcoords (LocalVariables|GetchosenTile)) (Utilities|Select :Index (Utilities|Select :Index _index :Option%200 "NewEnumerator0" :Option%201 "NewEnumerator1" :Option%202 "NewEnumerator2" :Option%203 "NewEnumerator3") :NewEnumerator0 "0.000000,1.000000,0.000000" :NewEnumerator1 "-1.000000,0.000000,0.000000" :NewEnumerator2 "0.000000,-1.000000,0.000000" :NewEnumerator3 "1.000000,0.000000, 0" :NewEnumerator8 "9999.000000, 0, 0")))) 0.0) (< (.X (Math|Vector|BreakVector (+ (Variables|/Game/Blueprints/bp_roomSquare.bp_roomSquare_C|Getcoords (LocalVariables|GetchosenTile)) (Utilities|Select :Index (Utilities|Select :Index _index :Option%200 "NewEnumerator0" :Option%201 "NewEnumerator1" :Option%202 "NewEnumerator2" :Option%203 "NewEnumerator3") :NewEnumerator0 "0.000000,1.000000,0.000000" :NewEnumerator1 "-1.000000,0.000000,0.000000" :NewEnumerator2 "0.000000,-1.000000,0.000000" :NewEnumerator3 "1.000000,0.000000, 0" :NewEnumerator8 "9999.000000, 0, 0")))) _returnvalue_3) (>= (.Y (Math|Vector|BreakVector (+ (Variables|/Game/Blueprints/bp_roomSquare.bp_roomSquare_C|Getcoords (LocalVariables|GetchosenTile)) (Utilities|Select :Index (Utilities|Select :Index _index :Option%200 "NewEnumerator0" :Option%201 "NewEnumerator1" :Option%202 "NewEnumerator2" :Option%203 "NewEnumerator3") :NewEnumerator0 "0.000000,1.000000,0.000000" :NewEnumerator1 "-1.000000,0.000000,0.000000" :NewEnumerator2 "0.000000,-1.000000,0.000000" :NewEnumerator3 "1.000000,0.000000, 0" :NewEnumerator8 "9999.000000, 0, 0")))) 0.0) (< (.Y (Math|Vector|BreakVector (+ (Variables|/Game/Blueprints/bp_roomSquare.bp_roomSquare_C|Getcoords (LocalVariables|GetchosenTile)) (Utilities|Select :Index (Utilities|Select :Index _index :Option%200 "NewEnumerator0" :Option%201 "NewEnumerator1" :Option%202 "NewEnumerator2" :Option%203 "NewEnumerator3") :NewEnumerator0 "0.000000,1.000000,0.000000" :NewEnumerator1 "-1.000000,0.000000,0.000000" :NewEnumerator2 "0.000000,-1.000000,0.000000" :NewEnumerator3 "1.000000,0.000000, 0" :NewEnumerator8 "9999.000000, 0, 0")))) _returnvalue_3))
          (bind _tile (CallFunction|GetTilefromCoords (+ (Variables|/Game/Blueprints/bp_roomSquare.bp_roomSquare_C|Getcoords (LocalVariables|GetchosenTile)) (Utilities|Select :Index (Utilities|Select :Index _index :Option%200 "NewEnumerator0" :Option%201 "NewEnumerator1" :Option%202 "NewEnumerator2" :Option%203 "NewEnumerator3") :NewEnumerator0 "0.000000,1.000000,0.000000" :NewEnumerator1 "-1.000000,0.000000,0.000000" :NewEnumerator2 "0.000000,-1.000000,0.000000" :NewEnumerator3 "1.000000,0.000000, 0" :NewEnumerator8 "9999.000000, 0, 0"))))
          (Utilities|Array|Add (LocalVariables|GetadjacentTiles) _tile)))
      (Utilities|Array|RemoveItem (LocalVariables|GetadjacentTiles) (Variables|Default|GetstartTile))
      (Utilities|Array|RemoveItem (LocalVariables|GetadjacentTiles) (Variables|Default|GetexitTile))
      (if (== (Utilities|Array|FindItem (Variables|Default|GetclosedList) _output_2) -1)
        (if (Variables|/Game/Blueprints/bp_roomSquare.bp_roomSquare_C|GetexitHere? _output_2)
          (CallFunction|AddExtraRooms)
          (else
            (LocalVariables|SetchosenAdjacentTile _output_2)
            (CallFunction|CreateDoors (LocalVariables|GetchosenTile) (LocalVariables|GetchosenAdjacentTile))
            (CallFunction|CreateDoors (LocalVariables|GetchosenAdjacentTile) (LocalVariables|GetchosenTile))
            (Utilities|Array|Add (Variables|Default|GetclosedList) (LocalVariables|GetchosenAdjacentTile))
            (Rendering|Material|SetMaterial (Variables|/Game/Blueprints/bp_roomSquare.bp_roomSquare_C|GetStaticMesh (LocalVariables|GetchosenAdjacentTile)) 0 "/Engine/MapTemplates/Materials/BasicAsset02.BasicAsset02")
            (CallFunction|UpdateTiles)
            (return)))
        (else
          (CallFunction|AddExtraRooms))))
    (:Is%20Not%20Valid
      (CallFunction|AddExtraRooms))))

(fn UpdateTiles
  (for _array_element (Variables|Default|GetroomTileArray)
    (Default|UpdateArrows _array_element)))

(fn GetRoomNumber
  (for _array_element (Variables|Default|GetroomTileArray)
    (if (> (Utilities|Array|Length (Variables|/Game/Blueprints/bp_roomSquare.bp_roomSquare_C|GetdoorArray _array_element)) 0)
      (Math|Integer|IncrementInt (LocalVariables|Getn))))
  (return (LocalVariables|Getn)))

(fn RemoveStartandEndfromClosedList
  (bind _closedlist (Variables|Default|GetclosedList))
  (Utilities|Array|RemoveItem _closedlist (Variables|Default|GetstartTile))
  (Utilities|Array|RemoveItem _closedlist (Variables|Default|GetexitTile)))

(fn DestroyRoomTileActors
  (for _array_element (Variables|Default|GetroomTileArray)
    (Actor|DestroyActor _array_element)
    (Utilities|Array|RemoveItem (Variables|Default|GetroomTileArray) _array_element))
  (Utilities|Array|Clear (Variables|Default|GetroomTileArray))
  (bind _asbp_ctlr_player (Utilities|Casting|CastTobp_ctlr_player (Game|GetPlayerController 0)))
  (Variables|/Game/Blueprints/controllers/bp_ctlr_player.bp_ctlr_player_C|SetroomTileArray _asbp_ctlr_player (Variables|Default|GetroomArray)))
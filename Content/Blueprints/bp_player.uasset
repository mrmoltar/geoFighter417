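; Player actor for a grid-based game that tracks moves, highlights nearby tiles and manages a draining power meter.
; On begin play and each tile move, it gathers neighboring tiles from the controller's flattened 2D grid array and toggles their radius flag and material.
; Tick drains power and sets active-power flags by thresholds.
; The construction script positions the spring-arm camera from pitch and depth settings.
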(event Custom|resetVars
  (Variables|Moves|Setmoves (Variables|moves|GetmovesDefault)))

(event Custom|moveToNewTile
  (CallFunction|UpdateSurroundingTilesMaterial true)
  (Utilities|Array|Clear (Variables|Default|GetsurroundingTiles))
  (CallFunction|GetSurroundingTiles 1)
  (CallFunction|UpdateSurroundingTilesMaterial false))

(event EventBeginPlay
  (Variables|Default|SetpreviousCoords (Variables|Default|GetcurrentCoords))
  (CallFunction|GetSurroundingTiles 1)
  (CallFunction|UpdateSurroundingTilesMaterial false))

(event Collision|EventActorBeginOverlap
  (params (OtherActor :type Actor%20Object%20Reference)))

(event EventTick
  (params (DeltaSeconds :type Float%20%28single-precision%29))
  (Utilities|IsValid (Variables|refs|GetplayerControllerRef)
    (:Is%20Valid
      (if (> (Variables|powerValueVars|GetpowerValue) 0.0)
        (Variables|powerValueVars|SetpowerValue (- (Variables|powerValueVars|GetpowerValue) (Variables|PowerValueVars|GetpowerValueDecrement)))
        ;[1 1 1] set active powers
        (for (_ _array_index) (Variables|Default|GetactivePowers)
          (Utilities|Array|SetArrayElem (Variables|Default|GetactivePowers) _array_index (> (Variables|powerValueVars|GetpowerValue) (Math|Conversions|ToFloat(Integer) (* (+ _array_index 1) 25)))))))))

(fn ConstructionScript
  (Transformation|SetRelativeRotation (Variables|Default|GetSpringArm) (Math|Rotator|MakeRotator 0.0 (* (Variables|Default|GetcameraPitch) -1.0) 0.0) false false)
  (Transformation|SetRelativeLocation (Variables|Default|GetCamera) (Math|Vector|MakeVector (* (Variables|Default|GetcameraDepth) -1.0) 0.0 0.0) false false))

(fn SetNewPowerValue
  (params (amountToAdd :type Float%20%28single-precision%29))
  (if (< (Variables|powerValueVars|GetpowerValue) (Variables|PowerValueVars|GetpowerValueMax))
    (bind _output_get (Variables|powerValueVars|SetpowerValue (+ (Variables|powerValueVars|GetpowerValue) amountToAdd)))
    (return _output_get)
    (else
      (return 0.0))))

(fn UpdateSurroundingTilesMaterial
  (params (resetToDefualtMaterial? :type Boolean))
  (if resetToDefualtMaterial?
    (for _array_element (Variables|Default|GetsurroundingTiles)
      (Utilities|IsValid _array_element
        (:Is%20Valid
          (Variables|/Game/Blueprints/bp_gridSquare.bp_gridSquare_C|SetinPlayerRadius? _array_element false)
          (Default|SetTiletoDefault _array_element))))
    (else
      (for _array_element_2 (Variables|Default|GetsurroundingTiles)
        (Utilities|IsValid 0
          (:Is%20Valid
            (Variables|/Game/Blueprints/bp_gridSquare.bp_gridSquare_C|SetinPlayerRadius? _array_element_2 true)
            (Default|SetTiletoPlayerRadiusMat _array_element_2)))))))

(fn GetSurroundingTiles
  (params (radius :type Integer))
  (bind (_returnvalue _returnvalue2) (Utilities|GetCurrentCoords))
  (bind _playercontrollerref (Variables|refs|GetplayerControllerRef))
  (bind _playercontrollerref_2 (Variables|refs|GetplayerControllerRef))
  (LocalVariables|SetR radius)
  (LocalVariables|SetX (- _returnvalue radius))
  (LocalVariables|SetY (- _returnvalue2 radius))
  (for _index (range 0 radius)
    (LocalVariables|Seti (+ (LocalVariables|Geti) _index)))
  (LocalVariables|SetlocalArea (* (LocalVariables|Geti) (LocalVariables|Geti)))
  (for _index_2 (range 0 (- (LocalVariables|Geti) 1))
    (bind _element (Utilities|Get2dArray (Variables|/Game/Blueprints/controllers/bp_ctlr_player.bp_ctlr_player_C|GetgridArray _playercontrollerref_2) (LocalVariables|GetX) (+ (LocalVariables|GetY) _index_2) (Variables|/Game/Blueprints/controllers/bp_ctlr_player.bp_ctlr_player_C|GetgridHorizontal _playercontrollerref_2))
      (:1
        (Utilities|IsValid _element
          (:Is%20Valid
            (Utilities|Array|Add (Variables|Default|GetsurroundingTiles) _element))
          (:Is%20Not%20Valid
            _))
        (for _index_3 (range 1 (- (LocalVariables|Geti) 1))
          (bind _element_2 (Utilities|Get2dArray (Variables|/Game/Blueprints/controllers/bp_ctlr_player.bp_ctlr_player_C|GetgridArray _playercontrollerref) (+ (LocalVariables|GetX) _index_3) (+ (LocalVariables|GetY) _index_2) (Variables|/Game/Blueprints/controllers/bp_ctlr_player.bp_ctlr_player_C|GetgridHorizontal _playercontrollerref))
            (:1
              (Utilities|IsValid _element_2
                (:Is%20Valid
                  (Utilities|Array|Add (Variables|Default|GetsurroundingTiles) _element_2)))))))))
  (return (Variables|Default|GetsurroundingTiles)))

(fn TileWithinRange?
  (params (OtherActor :type Actor%20Object%20Reference) (Radius :type Integer))
  (return (< (* Radius (Variables|/Game/Blueprints/controllers/bp_ctlr_player.bp_ctlr_player_C|GetmaxDistance (Variables|refs|GetplayerControllerRef))) (Transformation|GetDistanceTo OtherActor))))
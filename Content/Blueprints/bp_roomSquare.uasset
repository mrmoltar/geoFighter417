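; Square room tile Blueprint that visually marks its door directions and whether it is the start or exit room.
; On BeginPlay it loops over DoorArray and makes the matching north, east, south or west arrow visible for each entry.
; It then swaps the static mesh material for exit or start rooms, with exit taking priority when both flags are set.
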(event EventBeginPlay
  (bind _staticmesh (Variables|Default|GetStaticMesh))
  (Utilities|FlowControl|Sequence
    (:then_0
      (for _array_element (Variables|Default|GetdoorArray)
        (if (Utilities|Enum|Equal(Enum) _array_element "NewEnumerator0")
          (Rendering|SetVisibility (Variables|Default|GetNArrow) true false)
          (elif (Utilities|Enum|Equal(Enum) _array_element "NewEnumerator1")
            (Rendering|SetVisibility (Variables|Default|GetEArrow) true false)
            (elif (Utilities|Enum|Equal(Enum) _array_element "NewEnumerator2")
              (Rendering|SetVisibility (Variables|Default|GetSArrow) true false)
              (elif (Utilities|Enum|Equal(Enum) _array_element "NewEnumerator3")
                (Rendering|SetVisibility (Variables|Default|GetWArrow) true false)))))))
    (:then_1
      (if (Variables|Default|GetexitHere?)
        (Rendering|Material|SetMaterial _staticmesh 0 "/Engine/MapTemplates/Materials/BasicAsset01.BasicAsset01")
        (elif (Variables|Default|GetstartHere?)
          (Rendering|Material|SetMaterial _staticmesh 0 "/Game/materials/m_tileBasic4.m_tileBasic4"))))))

(event Collision|EventActorBeginOverlap
  (params (OtherActor :type Actor%20Object%20Reference)))

(event EventTick
  (params (DeltaSeconds :type Float%20%28single-precision%29)))

(fn ConstructionScript)
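; Room database Blueprint that loads numbered PNG room layouts from disk and catalogs them by door configuration.
; On BeginPlay it counts the images, clears its arrays, then checks four fixed edge pixels for the door grey to sort each room's pixels into one of fifteen N/E/S/W arrays.
; It also builds a color-code array that GetFeatureEnemyFromColor uses to translate a pixel color into an enemy or feature enum by index.
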(event EventBeginPlay
  (bind _roomimagenumber (CallFunction|GetRoomImageTotal))
  ;[1 1 1] break exec pin once levels are added!
  (CallFunction|ClearAllDoorArrays)
  (CallFunction|SortRoomImagesViaDoors _roomimagenumber)
  (Development|PrintString "Room images updated!")
  (Variables|COLORCODES|SetcolorCodesArray (Utilities|Array|MakeArray (Variables|COLORCODES|Getfloor_color) (Variables|COLORCODES|Getwall_color) (Variables|COLORCODES|Getdoor_Color) (Variables|COLORCODES|GetspringBoardN_color) (Variables|COLORCODES|GetspringBoardNE_color) (Variables|COLORCODES|GetspringBoardE_color) (Variables|COLORCODES|GetspringBoardSE_color) (Variables|COLORCODES|GetspringBoardS_color) (Variables|COLORCODES|GetspringBoardSW_color) (Variables|COLORCODES|GetspringBoardW_color) (Variables|COLORCODES|GetspringBoardNW_color) (Variables|COLORCODES|GetbombLauncherN_color) (Variables|COLORCODES|GetbombLauncherNE_color) (Variables|COLORCODES|GetbombLauncherE_color) (Variables|COLORCODES|GetbombLauncherSE_color) (Variables|COLORCODES|GetbombLauncherS_color) (Variables|COLORCODES|GetbombLauncherSW_color) (Variables|COLORCODES|GetbombLauncherW_color) (Variables|COLORCODES|GetbombLauncherNW_color) (Variables|COLORCODES|Getspike_color) (Variables|COLORCODES|Getpit_color) (Variables|COLORCODES|Getenemy_stationary_color) (Variables|COLORCODES|Getenemy_pursuer_color) (Variables|COLORCODES|Getenemy_runner_color))))

(fn ConstructionScript)

(fn SortRoomImagesViaDoors
  (params (LastIndex :type Integer))
  (bind _index (Utilities|FlowControl|ForLoopwithBreak 0 LastIndex :!label _label)
    (:LoopBody
      (Variables|DoorSortingVars|SetcurrentFileString (Utilities|String|Append (Variables|Default|GetroomImageFilepath) (Utilities|String|ToString(Integer) _index) ".png"))
      (if (.IsValid (Class|VictoryBPFunctionLibrary|VictoryLoadTexture2DfromFilePixels (Utilities|String|Append (Variables|Default|GetroomImageFilepath) (Utilities|String|ToString(Integer) _index) ".png") "PNG"))
        (Variables|DoorSortingVars|SetcurrentPixels (.OutPixels (Class|VictoryBPFunctionLibrary|VictoryLoadTexture2DfromFilePixels (Utilities|String|Append (Variables|Default|GetroomImageFilepath) (Utilities|String|ToString(Integer) _index) ".png") "PNG")))
        ;[1 1 1] N door
        (Variables|DoorSortingVars|SetnDoor? (Math|Vector|Equal(Vector) (Math|Vector|MakeVector (.R (Utilities|Struct|BreakLinearColor (Utilities|Array|Get(acopy) (.OutPixels (Class|VictoryBPFunctionLibrary|VictoryLoadTexture2DfromFilePixels (Utilities|String|Append (Variables|Default|GetroomImageFilepath) (Utilities|String|ToString(Integer) _index) ".png") "PNG")) 112))) (.G (Utilities|Struct|BreakLinearColor (Utilities|Array|Get(acopy) (.OutPixels (Class|VictoryBPFunctionLibrary|VictoryLoadTexture2DfromFilePixels (Utilities|String|Append (Variables|Default|GetroomImageFilepath) (Utilities|String|ToString(Integer) _index) ".png") "PNG")) 112))) (.B (Utilities|Struct|BreakLinearColor (Utilities|Array|Get(acopy) (.OutPixels (Class|VictoryBPFunctionLibrary|VictoryLoadTexture2DfromFilePixels (Utilities|String|Append (Variables|Default|GetroomImageFilepath) (Utilities|String|ToString(Integer) _index) ".png") "PNG")) 112)))) "127.000000,127.000000,127.000000" 0.0001))
        ;[1 1 1] W door
        (Variables|DoorSortingVars|SetwDoor? (Math|Vector|Equal(Vector) (Math|Vector|MakeVector (.R (Utilities|Struct|BreakLinearColor (Utilities|Array|Get(acopy) (.OutPixels (Class|VictoryBPFunctionLibrary|VictoryLoadTexture2DfromFilePixels (Utilities|String|Append (Variables|Default|GetroomImageFilepath) (Utilities|String|ToString(Integer) _index) ".png") "PNG")) 62))) (.G (Utilities|Struct|BreakLinearColor (Utilities|Array|Get(acopy) (.OutPixels (Class|VictoryBPFunctionLibrary|VictoryLoadTexture2DfromFilePixels (Utilities|String|Append (Variables|Default|GetroomImageFilepath) (Utilities|String|ToString(Integer) _index) ".png") "PNG")) 62))) (.B (Utilities|Struct|BreakLinearColor (Utilities|Array|Get(acopy) (.OutPixels (Class|VictoryBPFunctionLibrary|VictoryLoadTexture2DfromFilePixels (Utilities|String|Append (Variables|Default|GetroomImageFilepath) (Utilities|String|ToString(Integer) _index) ".png") "PNG")) 62)))) "127.000000,127.000000,127.000000" 0.0001))
        ;[1 1 1] E door
        (Variables|DoorSortingVars|SeteDoor? (Math|Vector|Equal(Vector) (Math|Vector|MakeVector (.R (Utilities|Struct|BreakLinearColor (Utilities|Array|Get(acopy) (.OutPixels (Class|VictoryBPFunctionLibrary|VictoryLoadTexture2DfromFilePixels (Utilities|String|Append (Variables|Default|GetroomImageFilepath) (Utilities|String|ToString(Integer) _index) ".png") "PNG")) 54))) (.G (Utilities|Struct|BreakLinearColor (Utilities|Array|Get(acopy) (.OutPixels (Class|VictoryBPFunctionLibrary|VictoryLoadTexture2DfromFilePixels (Utilities|String|Append (Variables|Default|GetroomImageFilepath) (Utilities|String|ToString(Integer) _index) ".png") "PNG")) 54))) (.B (Utilities|Struct|BreakLinearColor (Utilities|Array|Get(acopy) (.OutPixels (Class|VictoryBPFunctionLibrary|VictoryLoadTexture2DfromFilePixels (Utilities|String|Append (Variables|Default|GetroomImageFilepath) (Utilities|String|ToString(Integer) _index) ".png") "PNG")) 54)))) "127.000000,127.000000,127.000000" 0.0001))
        ;[1 1 1] S door
        (Variables|DoorSortingVars|SetsDoor? (Math|Vector|Equal(Vector) (Math|Vector|MakeVector (.R (Utilities|Struct|BreakLinearColor (Utilities|Array|Get(acopy) (.OutPixels (Class|VictoryBPFunctionLibrary|VictoryLoadTexture2DfromFilePixels (Utilities|String|Append (Variables|Default|GetroomImageFilepath) (Utilities|String|ToString(Integer) _index) ".png") "PNG")) 4))) (.G (Utilities|Struct|BreakLinearColor (Utilities|Array|Get(acopy) (.OutPixels (Class|VictoryBPFunctionLibrary|VictoryLoadTexture2DfromFilePixels (Utilities|String|Append (Variables|Default|GetroomImageFilepath) (Utilities|String|ToString(Integer) _index) ".png") "PNG")) 4))) (.B (Utilities|Struct|BreakLinearColor (Utilities|Array|Get(acopy) (.OutPixels (Class|VictoryBPFunctionLibrary|VictoryLoadTexture2DfromFilePixels (Utilities|String|Append (Variables|Default|GetroomImageFilepath) (Utilities|String|ToString(Integer) _index) ".png") "PNG")) 4)))) "127.000000,127.000000,127.000000" 0.0001))
        ;[1 1 1] Four Doors
        ;;[1 1 1] Only North & West & East & South Door?
        (if (Math|Boolean|ANDBoolean (Variables|DoorSortingVars|GetnDoor?) (Variables|DoorSortingVars|GetwDoor?) (Variables|DoorSortingVars|GeteDoor?) (Variables|DoorSortingVars|GetsDoor?))
          (Utilities|Array|Add (Variables|DEFAULTDOORS|GetnorthEastSouthWestDoors) (Utilities|Struct|Makestruct_room_pixelsAndDoors (Variables|DoorSortingVars|GetcurrentPixels)))
          (else
            ;[1 1 1] Three Doors
            ;;[1 1 1] Only North & West & East Door?
            (if (Math|Boolean|ANDBoolean (Variables|DoorSortingVars|GetnDoor?) (Variables|DoorSortingVars|GetwDoor?) (Variables|DoorSortingVars|GeteDoor?) (not (Variables|DoorSortingVars|GetsDoor?)))
              (Utilities|Array|Add (Variables|DEFAULTDOORS|GetnorthWestEastDoors) (Utilities|Struct|Makestruct_room_pixelsAndDoors (Variables|DoorSortingVars|GetcurrentPixels)))
              (else
                ;;[1 1 1] Only North & West & South Door?
                (if (Math|Boolean|ANDBoolean (Variables|DoorSortingVars|GetnDoor?) (Variables|DoorSortingVars|GetwDoor?) (Variables|DoorSortingVars|GetsDoor?) (not (Variables|DoorSortingVars|GeteDoor?)))
                  (Utilities|Array|Add (Variables|DEFAULTDOORS|GetnorthWestSouthDoors) (Utilities|Struct|Makestruct_room_pixelsAndDoors (Variables|DoorSortingVars|GetcurrentPixels)))
                  (else
                    ;;[1 1 1] Only West & East & South Door?
                    (if (Math|Boolean|ANDBoolean (Variables|DoorSortingVars|GetsDoor?) (Variables|DoorSortingVars|GetwDoor?) (Variables|DoorSortingVars|GeteDoor?) (not (Variables|DoorSortingVars|GetnDoor?)))
                      (Utilities|Array|Add (Variables|DEFAULTDOORS|GeteastSouthWestDoors) (Utilities|Struct|Makestruct_room_pixelsAndDoors (Variables|DoorSortingVars|GetcurrentPixels)))
                      (else
                        ;;[1 1 1] Only North & East & South Door?
                        (if (Math|Boolean|ANDBoolean (Variables|DoorSortingVars|GetsDoor?) (Variables|DoorSortingVars|GetnDoor?) (Variables|DoorSortingVars|GeteDoor?) (not (Variables|DoorSortingVars|GetwDoor?)))
                          (Utilities|Array|Add (Variables|DEFAULTDOORS|GetnorthEastSouthDoors) (Utilities|Struct|Makestruct_room_pixelsAndDoors (Variables|DoorSortingVars|GetcurrentPixels)))
                          (else
                            ;[1 1 1] Two Doors
                            ;;[1 1 1] Only North & West Door?
                            (if (Math|Boolean|ANDBoolean (Variables|DoorSortingVars|GetnDoor?) (Variables|DoorSortingVars|GetwDoor?) (not (Variables|DoorSortingVars|GeteDoor?)) (not (Variables|DoorSortingVars|GetsDoor?)))
                              (Utilities|Array|Add (Variables|DEFAULTDOORS|GetnorthWestDoors) (Utilities|Struct|Makestruct_room_pixelsAndDoors (Variables|DoorSortingVars|GetcurrentPixels)))
                              (else
                                ;;[1 1 1] Only North & East Door?
                                (if (Math|Boolean|ANDBoolean (Variables|DoorSortingVars|GetnDoor?) (Variables|DoorSortingVars|GeteDoor?) (not (Variables|DoorSortingVars|GetwDoor?)) (not (Variables|DoorSortingVars|GetsDoor?)))
                                  (Utilities|Array|Add (Variables|DEFAULTDOORS|GetnorthEastDoors) (Utilities|Struct|Makestruct_room_pixelsAndDoors (Variables|DoorSortingVars|GetcurrentPixels)))
                                  (else
                                    ;;[1 1 1] Only North & South Door?
                                    (if (Math|Boolean|ANDBoolean (Variables|DoorSortingVars|GetnDoor?) (Variables|DoorSortingVars|GetsDoor?) (not (Variables|DoorSortingVars|GeteDoor?)) (not (Variables|DoorSortingVars|GetwDoor?)))
                                      (Utilities|Array|Add (Variables|DEFAULTDOORS|GetnorthSouthDoors) (Utilities|Struct|Makestruct_room_pixelsAndDoors (Variables|DoorSortingVars|GetcurrentPixels)))
                                      (else
                                        ;;[1 1 1] Only West & East Door?
                                        (if (Math|Boolean|ANDBoolean (Variables|DoorSortingVars|GeteDoor?) (Variables|DoorSortingVars|GetwDoor?) (not (Variables|DoorSortingVars|GetnDoor?)) (not (Variables|DoorSortingVars|GetsDoor?)))
                                          (Utilities|Array|Add (Variables|DEFAULTDOORS|GeteastWestDoors) (Utilities|Struct|Makestruct_room_pixelsAndDoors (Variables|DoorSortingVars|GetcurrentPixels)))
                                          (else
                                            ;;[1 1 1] Only West & South Door?
                                            (if (Math|Boolean|ANDBoolean (Variables|DoorSortingVars|GetsDoor?) (Variables|DoorSortingVars|GetwDoor?) (not (Variables|DoorSortingVars|GetnDoor?)) (not (Variables|DoorSortingVars|GeteDoor?)))
                                              (Utilities|Array|Add (Variables|DEFAULTDOORS|GetsouthWestDoors) (Utilities|Struct|Makestruct_room_pixelsAndDoors (Variables|DoorSortingVars|GetcurrentPixels)))
                                              (else
                                                ;;[1 1 1] Only East & South Door?
                                                (if (Math|Boolean|ANDBoolean (Variables|DoorSortingVars|GeteDoor?) (Variables|DoorSortingVars|GetsDoor?) (not (Variables|DoorSortingVars|GetnDoor?)) (not (Variables|DoorSortingVars|GetwDoor?)))
                                                  (Utilities|Array|Add (Variables|DEFAULTDOORS|GeteastSouthDoors) (Utilities|Struct|Makestruct_room_pixelsAndDoors (Variables|DoorSortingVars|GetcurrentPixels)))
                                                  (else
                                                    ;[1 1 1] One Door
                                                    ;;[1 1 1] Only North Door?
                                                    (if (Math|Boolean|ANDBoolean (Variables|DoorSortingVars|GetnDoor?) (not (Variables|DoorSortingVars|GetwDoor?)) (not (Variables|DoorSortingVars|GeteDoor?)) (not (Variables|DoorSortingVars|GetsDoor?)))
                                                      (Utilities|Array|Add (Variables|DEFAULTDOORS|GetnorthDoors) (Utilities|Struct|Makestruct_room_pixelsAndDoors (Variables|DoorSortingVars|GetcurrentPixels)))
                                                      (else
                                                        ;;[1 1 1] Only West Door?
                                                        (if (Math|Boolean|ANDBoolean (Variables|DoorSortingVars|GetwDoor?) (not (Variables|DoorSortingVars|GetnDoor?)) (not (Variables|DoorSortingVars|GeteDoor?)) (not (Variables|DoorSortingVars|GetsDoor?)))
                                                          (Utilities|Array|Add (Variables|DEFAULTDOORS|GetwestDoors) (Utilities|Struct|Makestruct_room_pixelsAndDoors (Variables|DoorSortingVars|GetcurrentPixels)))
                                                          (else
                                                            ;;[1 1 1] Only East Door?
                                                            (if (Math|Boolean|ANDBoolean (Variables|DoorSortingVars|GeteDoor?) (not (Variables|DoorSortingVars|GetwDoor?)) (not (Variables|DoorSortingVars|GetnDoor?)) (not (Variables|DoorSortingVars|GetsDoor?)))
                                                              (Utilities|Array|Add (Variables|DEFAULTDOORS|GeteastDoors) (Utilities|Struct|Makestruct_room_pixelsAndDoors (Variables|DoorSortingVars|GetcurrentPixels)))
                                                              (else
                                                                ;;[1 1 1] Only South Door?
                                                                (if (Math|Boolean|ANDBoolean (Variables|DoorSortingVars|GetsDoor?) (not (Variables|DoorSortingVars|GetwDoor?)) (not (Variables|DoorSortingVars|GeteDoor?)) (not (Variables|DoorSortingVars|GetnDoor?)))
                                                                  (Utilities|Array|Add (Variables|DEFAULTDOORS|GetsouthDoors) (Utilities|Struct|Makestruct_room_pixelsAndDoors (Variables|DoorSortingVars|GetcurrentPixels)))
                                                                  (else
                                                                    (Development|PrintString "ERROR FINDING DOORS")))))))))))))))))))))))))))))))
        (else
          (Development|PrintString (Utilities|String|Append (Utilities|String|ToString(Integer) (Variables|Default|GetroomImageNumber)) " total rooms."))
          (goto _label Break))))))

(fn ClearAllDoorArrays
  (Utilities|Array|Clear (Variables|DEFAULTDOORS|GetnorthDoors))
  (Utilities|Array|Clear (Variables|DEFAULTDOORS|GeteastDoors))
  (Utilities|Array|Clear (Variables|DEFAULTDOORS|GetsouthDoors))
  (Utilities|Array|Clear (Variables|DEFAULTDOORS|GetsouthDoors))
  (Utilities|Array|Clear (Variables|DEFAULTDOORS|GetwestDoors))
  (Utilities|Array|Clear (Variables|DEFAULTDOORS|GetnorthEastDoors))
  (Utilities|Array|Clear (Variables|DEFAULTDOORS|GetnorthEastSouthDoors))
  (Utilities|Array|Clear (Variables|DEFAULTDOORS|GetnorthEastSouthWestDoors))
  (Utilities|Array|Clear (Variables|DEFAULTDOORS|GeteastSouthDoors))
  (Utilities|Array|Clear (Variables|DEFAULTDOORS|GeteastSouthWestDoors))
  (Utilities|Array|Clear (Variables|DEFAULTDOORS|GetsouthWestDoors))
  (Utilities|Array|Clear (Variables|DEFAULTDOORS|GetnorthSouthDoors))
  (Utilities|Array|Clear (Variables|DEFAULTDOORS|GeteastWestDoors))
  (Utilities|Array|Clear (Variables|DEFAULTDOORS|GetnorthWestEastDoors))
  (Utilities|Array|Clear (Variables|DEFAULTDOORS|GetnorthWestSouthDoors))
  (Utilities|Array|Clear (Variables|DEFAULTDOORS|GetnorthWestDoors)))

(fn GetFeature/EnemyfromColor
  (params (color :type Linear%20Color%20Structure))
  (bind (_r _g _b) (Math|Color|BreakColor color))
  (for (_array_element _array_index) (Variables|COLORCODES|GetcolorCodesArray)
    (if (Math|Vector|Equal(Vector) _array_element (Math|Vector|MakeVector _r _g _b) 0.0001)
      (bind _output_get (LocalVariables|SetenemyOrFeature (Utilities|Enum|ByteToEnume_enemiesAndFeatures (Math|Conversions|ToByte(Integer) _array_index))))
      (return true _output_get _array_element _array_index)))
  (return false "NewEnumerator1" "0, 0, 0" 0))

(fn GetRoomImageTotal
  (bind _roomimagenumber (Variables|Default|GetroomImageNumber))
  (while (.IsValid (Class|VictoryBPFunctionLibrary|VictoryLoadTexture2DfromFilePixels (Utilities|String|Append (Variables|Default|GetroomImageFilepath) (Utilities|String|ToString(Integer) (Variables|Default|GetroomImageNumber)) ".png") "PNG"))
    (Math|Integer|IncrementInt _roomimagenumber))
  (return _roomimagenumber))
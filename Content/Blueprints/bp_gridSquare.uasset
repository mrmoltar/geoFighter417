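; Grid tile actor that displays its coordinates and highlights under the cursor.
; BeginPlay randomly picks one of two base materials as the default, zeroes X if it equals the player controller's GridHorizontal, and writes the coordinate label.
; Cursor exit restores either the player-radius or default material, based on InPlayerRadius.
; Mesh begin-overlap sets PlayerHere according to whether the other actor is bp_player, with no end-overlap reset.
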(event OnComponentBeginOverlap(StaticMesh)
  (params (OverlappedComponent :type Primitive%20Component%20Object%20Reference) (OtherActor :type Actor%20Object%20Reference) (OtherComp :type Primitive%20Component%20Object%20Reference) (OtherBodyIndex :type Integer) (bFromSweep :type Boolean) (SweepResult :type Hit%20Result%20Structure%20%28by%20ref%29))
  (Utilities|Casting|CastTobp_player OtherActor
    (:then
      (Variables|Default|SetplayerHere? true))
    (:CastFailed
      (Variables|Default|SetplayerHere? false))))

(event OnEndCursorOver(StaticMesh)
  (params (TouchedComponent :type Primitive%20Component%20Object%20Reference))
  (if (Variables|Default|GetinPlayerRadius?)
    (CallFunction|SetTiletoPlayerRadiusMat)
    (else
      (CallFunction|SetTiletoDefault))))

(event OnBeginCursorOver(StaticMesh)
  (params (TouchedComponent :type Primitive%20Component%20Object%20Reference))
  (Rendering|Material|SetMaterial TouchedComponent 0 "/Engine/MapTemplates/Materials/BasicAsset01.BasicAsset01"))

(event EventBeginPlay
  (bind _staticmesh (Variables|Default|GetStaticMesh))
  (Utilities|FlowControl|Sequence
    (:then_0
      (if (Math|Random|RandomBool)
        (Rendering|Material|SetMaterial _staticmesh 0 "/Game/materials/m_tileBasic1.m_tileBasic1")
        (else
          (Rendering|Material|SetMaterial _staticmesh 0 "/Game/materials/m_tileBasic2.m_tileBasic2")))
      (Variables|Default|SetdefaultMaterial (Rendering|Material|GetMaterial (Variables|Default|GetStaticMesh) 0)))
    (:then_1
      (bind _asbp_ctlr_player (Utilities|Casting|CastTobp_ctlr_player (Game|GetPlayerController 0)))
      (if (== (.x (Variables|Default|GetcurrentCoords)) (Math|Conversions|ToFloat(Integer) (Variables|/Game/Blueprints/controllers/bp_ctlr_player.bp_ctlr_player_C|GetgridHorizontal _asbp_ctlr_player)))
        (Variables|Default|SetcurrentCoords (Math|Vector|MakeVector 0.0 (.y (Variables|Default|GetcurrentCoords)) 0.0))))
    (:then_2
      (Rendering|Components|TextRender|SetText (Variables|Default|GetcoordinateText) (Utilities|Text|ToText(String) (Utilities|String|Append (Utilities|String|ToString(Integer) (Math|Float|Floor (.x (Variables|Default|GetcurrentCoords)))) "." (Utilities|String|ToString(Integer) (Math|Float|Floor (.y (Variables|Default|GetcurrentCoords))))))))))

(event Collision|EventActorBeginOverlap
  (params (OtherActor :type Actor%20Object%20Reference)))

(event EventTick
  (params (DeltaSeconds :type Float%20%28single-precision%29)))

(fn ConstructionScript)

(fn SetTiletoDefault
  (Rendering|Material|SetMaterial (Variables|Default|GetStaticMesh) 0 (Variables|Default|GetdefaultMaterial))
  (return))

(fn SetTiletoPlayerRadiusMat
  (Rendering|Material|SetMaterial (Variables|Default|GetStaticMesh) 0 (Variables|Default|GetinPlayerRadiusMaterial))
  (return))
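; Rhythm controller that runs the game's beat clock, counting beats and measures after an audible countdown shown on the HUD.
; A rhythm timeline cues the music controller on beats 1/3 and 2/4, resetting player variables on 1/3.
; Tick sets global time dilation to BPM/60 to scale timeline tempo, and derives RhythmState from timeline-value tolerance windows.
; Separate helpers detect whole-to-sixteenth note crossings from song position and crotchet length.
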(event EventTick
  (params (DeltaSeconds :type Float%20%28single-precision%29))
  (bind _rhythmvalue (Variables|Default|GetrhythmValue))
  (Utilities|FlowControl|Sequence
    (:then_0
      ;[1 1 1] set time dilation based on BPM. This slows or speeds up the timelines
      (Utilities|Time|SetGlobalTimeDilation (/ (Variables|Default|Getbpm) 6e+01)))
    (:then_1
      ;[1 1 1] set rhythm state
      (if (Math|Float|NearlyEqual(Float) _rhythmvalue 0.5 0.05)
        (Variables|Default|SetrhythmState "NewEnumerator0")
        (elif (or (Math|Float|NearlyEqual(Float) _rhythmvalue 0.0 0.01) (Math|Float|NearlyEqual(Float) _rhythmvalue 1.0 0.01))
          (Variables|Default|SetrhythmState "NewEnumerator1")
          (elif (Math|Float|NearlyEqual(Float) _rhythmvalue 0.5 0.2)
            (Variables|Default|SetrhythmState "NewEnumerator2")
            (else
              (Variables|Default|SetrhythmState "NewEnumerator3"))))))))

(event EventBeginPlay
  (bind _playerctlrref (Variables|Default|GetplayerCtlrRef))
  (bind _musiccontrollerref (Variables|/Game/Blueprints/controllers/bp_ctlr_player.bp_ctlr_player_C|GetmusicControllerRef _playerctlrref))
  (Variables|Default|SetinitialSeconds (.Seconds (Class|GameplayStatics|GetAccurateRealTime)))
  ;[1 1 1] countdown timeline
  (bind _newtrack_3 (Timeline|countdown Play)
    (:Update
      (Variables|Default|SetcountdownFloat _newtrack_3)
      (Variables|/Game/Blueprints/widgets/w_hud.w_hud_C|Setcountdown (Variables|/Game/Blueprints/controllers/bp_ctlr_player.bp_ctlr_player_C|GethudRef (Variables|Default|GetplayerCtlrRef)) _newtrack_3))
    (:Finished
      ;[1 1 1] begin rhythm timeline (looped)
      (bind _newtrack_0 (Timeline|rhythmTimeline Play)
        (:Update
          (Variables|Default|SetrhythmValue _newtrack_0))
        (:Finished
          ;[1 1 1] ++ total number of measures (4 beats = 1 measure)
          (Math|Integer|IncrementInt (Variables|Default|GetmeasureNumber)))
        (:1%20&%203
          (Default|1&3 _musiccontrollerref)
          ;[1 1 1] reset player moves to default values
          (Default|ResetVars (Variables|/Game/Blueprints/controllers/bp_ctlr_player.bp_ctlr_player_C|GetplayerRef (Variables|Default|GetplayerCtlrRef)))
          ;[1 1 1] ++ total number of beats
          (Math|Float|IncrementFloat (Variables|Default|GetbeatNumber) :!label _label))
        (:2%20&%204
          (Default|2&4 _musiccontrollerref)
          (goto _label))))
    (:NewTrack_4
      ;;[1 1 1] every beat of countdown - play sound
      (Audio|PlaySound2D "/Game/Blueprints/sounds/DNC_Hat_4.DNC_Hat_4"))))

(fn ConstructionScript)

(fn GetSubdivision
  (params (subdivision :type e_beatSubdivision%20Enum :default "NewEnumerator0"))
  (bind _returnvalue (Utilities|Select :Index subdivision :NewEnumerator0 4.0 :NewEnumerator1 2.0 :NewEnumerator2 1.0 :NewEnumerator3 0.5 :NewEnumerator4 0.25))
  (bind _lastwholenote (Variables|PreviousBeats|GetlastWholeNote))
  (bind _lasthalfnote (Variables|PreviousBeats|GetlastHalfNote))
  (bind _lastquarternote (Variables|PreviousBeats|GetlastQuarterNote))
  (bind _lasteighthnote (Variables|PreviousBeats|GetlastEighthNote))
  (bind _lastsixteenthnote (Variables|PreviousBeats|GetlastSixteenthNote))
  (bind _crotchet (Variables|Default|Getcrotchet))
  (bind _returnvalue_2 (* _crotchet _returnvalue))
  (bind _returnvalue_3 (Utilities|Select :Index subdivision :NewEnumerator0 _lastwholenote :NewEnumerator1 _lasthalfnote :NewEnumerator2 _lastquarternote :NewEnumerator3 _lasteighthnote :NewEnumerator4 _lastsixteenthnote))
  (bind _returnvalue_4 (+ _returnvalue_3 _returnvalue_2))
  (if (> (+ (Variables|Default|GetsongPosition) (Utilities|Time|GetWorldDeltaSeconds)) _returnvalue_4)
    (return true _returnvalue_4)
    (else
      (return false 0.0))))
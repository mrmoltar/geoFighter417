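; Level feature controller that spawns and drives grid hazards and gadgets in time with the rhythm.
; Spawn functions place floor spikes, springboards, bomb launchers and pits on player controller grid tiles, optionally randomizing direction, and track them in arrays.
; checkTriggers compares each feature's trigger values to the rhythm controller's RhythmValue within a tolerance, firing its action or counting down bomb timers to explosion.
; DestroyAllFeatures destroys the tracked actors.
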(event Custom|checkTriggers
  (CallFunction|CheckArrayforTriggers "NewEnumerator0")
  (CallFunction|CheckArrayforTriggers "NewEnumerator1")
  (CallFunction|CheckArrayforTriggers "NewEnumerator2")
  (CallFunction|CheckArrayforTriggers "NewEnumerator4"))

(event EventBeginPlay)

(event Collision|EventActorBeginOverlap
  (params (OtherActor :type Actor%20Object%20Reference)))

(event EventTick
  (params (DeltaSeconds :type Float%20%28single-precision%29)))

(fn ConstructionScript)

(fn SpawnFloorSpikes
  (params (X :type Integer) (Y :type Integer))
  (bind _playercontrollerref (Variables|Default|GetplayerControllerRef))
  (bind _playercontrollerref_2 (Variables|Default|GetplayerControllerRef))
  (bind _element (Utilities|Get2dArray (Variables|/Game/Blueprints/controllers/bp_ctlr_player.bp_ctlr_player_C|GetgridArray _playercontrollerref_2) X Y (Variables|/Game/Blueprints/controllers/bp_ctlr_player.bp_ctlr_player_C|GetgridHorizontal _playercontrollerref_2))
    (:1
      (bind _returnvalue (Game|SpawnActorfromClass "/Game/Blueprints/levelFeatures/bp_floorSpikes.bp_floorSpikes_C" (Math|Transform|MakeTransform (Math|Vector|MakeVector (.x (Transformation|GetWorldLocation (Variables|/Game/Blueprints/bp_gridSquare.bp_gridSquare_C|GetDefaultSceneRoot _element))) (.y (Transformation|GetWorldLocation (Variables|/Game/Blueprints/bp_gridSquare.bp_gridSquare_C|GetDefaultSceneRoot _element))) 1e+01) "0, 0, 0" "1,1,1") "Undefined" 0 _element (Variables|/Game/Blueprints/controllers/bp_ctlr_player.bp_ctlr_player_C|GetrhythmControllerRef _playercontrollerref) _playercontrollerref 0))
      (Utilities|Array|Add (Variables|Default|GetfloorSpikeRefs) _returnvalue)
      (return _returnvalue))))

(fn SpawnSpringBoard
  (params (X :type Integer) (Y :type Integer) (randomizeDirection? :type Boolean) (direction :type e_8directions%20Enum :default "NewEnumerator0"))
  (bind _playercontrollerref (Variables|Default|GetplayerControllerRef))
  (bind _playercontrollerref_2 (Variables|Default|GetplayerControllerRef))
  (bind _playercontrollerref_3 (Variables|Default|GetplayerControllerRef))
  (bind _element (Utilities|Get2dArray (Variables|/Game/Blueprints/controllers/bp_ctlr_player.bp_ctlr_player_C|GetgridArray _playercontrollerref) X Y (Variables|/Game/Blueprints/controllers/bp_ctlr_player.bp_ctlr_player_C|GetgridHorizontal _playercontrollerref))
    (:1
      (if randomizeDirection?
        (bind _returnvalue (Game|SpawnActorfromClass "/Game/Blueprints/levelFeatures/bp_springBoard.bp_springBoard_C" (Math|Transform|MakeTransform (Math|Vector|MakeVector (.x (Transformation|GetWorldLocation (Variables|/Game/Blueprints/bp_gridSquare.bp_gridSquare_C|GetDefaultSceneRoot _element))) (.y (Transformation|GetWorldLocation (Variables|/Game/Blueprints/bp_gridSquare.bp_gridSquare_C|GetDefaultSceneRoot _element))) 1e+01) "0, 0, 0" "1,1,1") "Undefined" 0 (Utilities|Select :Index (Math|Random|RandomInteger 7) :Option%200 "NewEnumerator0" :Option%201 "NewEnumerator4" :Option%202 "NewEnumerator1" :Option%203 "NewEnumerator5" :Option%204 "NewEnumerator2" :Option%205 "NewEnumerator6" :Option%206 "NewEnumerator3" :Option%207 "NewEnumerator7") (Variables|/Game/Blueprints/controllers/bp_ctlr_player.bp_ctlr_player_C|GetrhythmControllerRef _playercontrollerref_2) _playercontrollerref_2 0 _element 0))
        (Utilities|Array|Add (Variables|Default|GetspringBoardRefs) _returnvalue)
        (return _returnvalue)
        (else
          (bind _returnvalue_2 (Game|SpawnActorfromClass "/Game/Blueprints/levelFeatures/bp_springBoard.bp_springBoard_C" (Math|Transform|MakeTransform (Math|Vector|MakeVector (.x (Transformation|GetWorldLocation (Variables|/Game/Blueprints/bp_gridSquare.bp_gridSquare_C|GetDefaultSceneRoot _element))) (.y (Transformation|GetWorldLocation (Variables|/Game/Blueprints/bp_gridSquare.bp_gridSquare_C|GetDefaultSceneRoot _element))) 1e+01) "0, 0, 0" "1,1,1") "Undefined" 0 direction (Variables|/Game/Blueprints/controllers/bp_ctlr_player.bp_ctlr_player_C|GetrhythmControllerRef _playercontrollerref_3) _playercontrollerref_3 0 _element 0))
          (Utilities|Array|Add (Variables|Default|GetspringBoardRefs) _returnvalue_2)
          (return _returnvalue_2))))))

(fn SpawnBombLauncher
  (params (X :type Integer) (Y :type Integer) (randomizeDirection? :type Boolean) (direction :type e_cardinalDirections%20Enum :default "NewEnumerator0"))
  (bind _playercontrollerref (Variables|Default|GetplayerControllerRef))
  (bind _playercontrollerref_2 (Variables|Default|GetplayerControllerRef))
  (bind _playercontrollerref_3 (Variables|Default|GetplayerControllerRef))
  (bind _element (Utilities|Get2dArray (Variables|/Game/Blueprints/controllers/bp_ctlr_player.bp_ctlr_player_C|GetgridArray _playercontrollerref_3) X Y (Variables|/Game/Blueprints/controllers/bp_ctlr_player.bp_ctlr_player_C|GetgridHorizontal _playercontrollerref_3))
    (:1
      (if randomizeDirection?
        (bind _returnvalue (Game|SpawnActorfromClass "/Game/Blueprints/levelFeatures/bp_bombLauncher.bp_bombLauncher_C" (Math|Transform|MakeTransform (Math|Vector|MakeVector (.x (Transformation|GetWorldLocation (Variables|/Game/Blueprints/bp_gridSquare.bp_gridSquare_C|GetDefaultSceneRoot _element))) (.y (Transformation|GetWorldLocation (Variables|/Game/Blueprints/bp_gridSquare.bp_gridSquare_C|GetDefaultSceneRoot _element))) 0.0) "0, 0, 0" "1,1,1") "Undefined" 0 (Utilities|Select :Index (Math|Random|RandomInteger 3) :Option%200 "NewEnumerator0" :Option%201 "NewEnumerator1" :Option%202 "NewEnumerator2" :Option%203 "NewEnumerator3") (Variables|/Game/Blueprints/controllers/bp_ctlr_player.bp_ctlr_player_C|GetrhythmControllerRef _playercontrollerref) _playercontrollerref _element 0))
        (Utilities|Array|Add (Variables|Default|GetbombLauncherRefs) _returnvalue)
        (return _returnvalue)
        (else
          (bind _returnvalue_2 (Game|SpawnActorfromClass "/Game/Blueprints/levelFeatures/bp_bombLauncher.bp_bombLauncher_C" (Math|Transform|MakeTransform (Math|Vector|MakeVector (.x (Transformation|GetWorldLocation (Variables|/Game/Blueprints/bp_gridSquare.bp_gridSquare_C|GetDefaultSceneRoot _element))) (.y (Transformation|GetWorldLocation (Variables|/Game/Blueprints/bp_gridSquare.bp_gridSquare_C|GetDefaultSceneRoot _element))) 0.0) "0, 0, 0" "1,1,1") "Undefined" 0 direction (Variables|/Game/Blueprints/controllers/bp_ctlr_player.bp_ctlr_player_C|GetrhythmControllerRef _playercontrollerref_2) _playercontrollerref_2 0 0))
          (Utilities|Array|Add (Variables|Default|GetbombLauncherRefs) 0)
          (return _returnvalue_2))))))

(fn SpawnPit
  (params (X :type Integer) (Y :type Integer))
  (bind _playercontrollerref (Variables|Default|GetplayerControllerRef))
  (bind _element (Utilities|Get2dArray (Variables|/Game/Blueprints/controllers/bp_ctlr_player.bp_ctlr_player_C|GetgridArray _playercontrollerref) X Y (Variables|/Game/Blueprints/controllers/bp_ctlr_player.bp_ctlr_player_C|GetgridHorizontal _playercontrollerref))
    (:1
      (bind _returnvalue (Game|SpawnActorfromClass "/Game/Blueprints/levelFeatures/bp_pit.bp_pit_C" (Math|Transform|MakeTransform (Math|Vector|MakeVector (.x (Transformation|GetWorldLocation (Variables|/Game/Blueprints/bp_gridSquare.bp_gridSquare_C|GetDefaultSceneRoot _element))) (.y (Transformation|GetWorldLocation (Variables|/Game/Blueprints/bp_gridSquare.bp_gridSquare_C|GetDefaultSceneRoot _element))) 1e+01) "0, 0, 0" "1,1,1") "Undefined" 0 "0.000000,0.000000,0.000000" _element (Variables|Default|GetplayerControllerRef) 0))
      (Utilities|Array|Add (Variables|Default|GetpitRefs) _returnvalue)
      (return _returnvalue))))

(fn CheckArrayforTriggers
  (params (levelFeature :type e_levelFeatures%20Enum :default "NewEnumerator0"))
  (switch Utilities|FlowControl|Switch|Switchone_levelFeatures levelFeature
    (:NewEnumerator0
      (for _array_element (Variables|Default|GetspringBoardRefs)
        (Utilities|TestTrigger (Variables|/Game/Blueprints/levelFeatures/bp_springBoard.bp_springBoard_C|GetbeatTrigger _array_element)
          (:true
            (Default|SpringPlayer _array_element)))))
    (:NewEnumerator1
      (for _array_element_2 (Variables|Default|GetfloorSpikeRefs)
        (Utilities|TestTrigger (Variables|/Game/Blueprints/levelFeatures/bp_floorSpikes.bp_floorSpikes_C|GetbeatTrigger _array_element_2)
          (:true
            (Default|ExtendSpikes _array_element_2))
          (:false
            (Utilities|TestTrigger (Variables|/Game/Blueprints/levelFeatures/bp_floorSpikes.bp_floorSpikes_C|GetbeatRetract _array_element_2)
              (:true
                (Default|RetractSpikes _array_element_2)))))))
    (:NewEnumerator2
      (for _array_element_3 (Variables|Default|GetbombLauncherRefs)
        (Utilities|TestTrigger (Variables|/Game/Blueprints/levelFeatures/bp_bombLauncher.bp_bombLauncher_C|GetturnValue _array_element_3)
          (:true
            (Default|Rotate _array_element_3))
          (:false
            (Utilities|TestTrigger (Variables|/Game/Blueprints/levelFeatures/bp_bombLauncher.bp_bombLauncher_C|GetshootValue _array_element_3)
              (:true
                (Default|Shoot _array_element_3 (Variables|/Game/Blueprints/levelFeatures/bp_bombLauncher.bp_bombLauncher_C|GetbombDistance _array_element_3))))))))
    (:NewEnumerator4
      (Utilities|TestTrigger (.explosionTrigger (Utilities|GetClassDefaults "/Game/Blueprints/levelFeatures/bp_bomb.bp_bomb_C"))
        (:true
          (for _array_element_4 (Variables|Default|GetbombRefs)
            (bind _result (Math|Integer|DecrementInt (Variables|/Game/Blueprints/levelFeatures/bp_bomb.bp_bomb_C|Gettimer _array_element_4))
              (:%20%20
                (if (<= _result 0)
                  (Default|Explode _array_element_4)
                  (Actor|DestroyActor _array_element_4)))))
          (for (_array_element_5 _array_index) (Variables|Default|GetbombRefs)
            (Utilities|IsValid _array_element_5
              (:Is%20Not%20Valid
                (Utilities|Array|RemoveIndex (Variables|Default|GetbombRefs) _array_index)))))))))

(fn DestroyAllFeatures
  (for _array_element (Variables|Default|GetfloorSpikeRefs)
    (Actor|DestroyActor _array_element))
  (for _array_element_2 (Variables|Default|GetspringBoardRefs)
    (Actor|DestroyActor _array_element_2))
  (for _array_element_3 (Variables|Default|GetbombLauncherRefs)
    (Actor|DestroyActor _array_element_3))
  (for _array_element_4 (Variables|Default|GetbombRefs)
    (Actor|DestroyActor _array_element_4)
    (for _array_element_5 (Variables|Default|GetpitRefs)
      (Actor|DestroyActor _array_element_5))))
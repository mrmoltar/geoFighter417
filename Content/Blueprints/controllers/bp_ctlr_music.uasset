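; Music controller Blueprint that plays the game's rhythmic percussion and combat sound effects as 2D sounds.
; Beat events trigger kick on beats 1 and 3, snare on 2 and 4, and hi-hat on eighth notes.
; Three player attack events and an enemy-type-selected death function share a concurrency setting.
; A BGM helper exists, but its only call is disconnected, alongside other unused experimental nodes.
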(event Custom|1%20&%203
  (Audio|PlaySound2D (Variables|Default|GetkickDrum1)))

(event Custom|Player%20Attack%201
  (Audio|PlaySound2D "/Engine/EditorSounds/GamePreview/PossessPlayer_Cue.PossessPlayer_Cue" 1.0 1.0 0.0 "/Game/sounds/bp_concurrency_default.bp_concurrency_default"))

(event Custom|Player%20Attack%203
  (Audio|PlaySound2D "/Engine/VREditor/Sounds/VR_ungrab_Cue.VR_ungrab_Cue" 1.0 1.2 0.0 "/Game/sounds/bp_concurrency_default.bp_concurrency_default"))

(event Custom|8th%20Notes
  (Audio|PlaySound2D (Variables|Default|GetHIHat1) 0.5 2.0))

(event Custom|2%20&%204
  (Audio|PlaySound2D (Variables|Default|Getsnare1)))

(event Custom|Player%20Attack%202
  (Audio|PlaySound2D "/Engine/VREditor/Sounds/VR_teleport.VR_teleport" 1.0 1.2 0.0 "/Game/sounds/bp_concurrency_default.bp_concurrency_default"))

(event EventBeginPlay)

(fn ConstructionScript)

(fn EnemyDeath
  (params (enemyType :type e_enemyTypes%20Enum :default "NewEnumerator0"))
  (Audio|PlaySound2D (Utilities|Select :Index enemyType :NewEnumerator0 (Variables|Default|GetconeDeath) :NewEnumerator1 (Variables|Default|GetcubeDeath) :NewEnumerator2 (Variables|Default|GetcylDeath)) 1.0 1.0 0.0 "/Game/sounds/bp_concurrency_default.bp_concurrency_default")
  (return))

(fn PlayBGM
  (params (Sound :type Sound%20Base%20Object%20Reference))
  (Audio|PlaySound2D Sound 0.2))
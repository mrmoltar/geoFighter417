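; Enemy controller for a grid-based rhythm game that spawns, tracks and destroys cone, cube and cylinder enemies.
; SpawnEnemyAtLocation picks random tiles, recursively retries impassable or occupied ones, then registers each enemy on its tile and in overall and per-type arrays.
; Once the countdown is zero, Tick watches the rhythm controller's Enemy Hit state, making cones choose tiles and cubes attack at opposite ends of the rhythm value.
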(event Custom|spawnRandomEnemies
  (for _index (range 0 3)
    (CallFunction|SpawnEnemyatLocation "/Game/Blueprints/enemies/bp_enemy_cone.bp_enemy_cone_C" 0 0 "NewEnumerator0" false)
    (CallFunction|SpawnEnemyatLocation "/Game/Blueprints/enemies/bp_enemy_cube.bp_enemy_cube_C" 0 0 "NewEnumerator1" false)))

(event EventBeginPlay)

(event EventTick
  (params (DeltaSeconds :type Float%20%28single-precision%29))
  (Utilities|IsValid (Variables|Default|GetrhythmControllerRef)
    (:Is%20Valid
      (if (== (Variables|/Game/Blueprints/controllers/bp_ctlr_rhythm.bp_ctlr_rhythm_C|GetcountdownFloat (Variables|Default|GetrhythmControllerRef)) 0.0)
        (if (Math|Float|NearlyEqual(Float) (Variables|/Game/Blueprints/controllers/bp_ctlr_rhythm.bp_ctlr_rhythm_C|GetrhythmValue (Variables|Default|GetrhythmControllerRef)) 0.0 0.01)
          (switch Utilities|FlowControl|Switch|Switchone_rhythmState (Variables|/Game/Blueprints/controllers/bp_ctlr_rhythm.bp_ctlr_rhythm_C|GetrhythmState (Variables|Default|GetrhythmControllerRef))
            (:NewEnumerator1
              (bind _outactors (Actor|GetAllActorsOfClass "/Game/Blueprints/enemies/bp_enemy_cone.bp_enemy_cone_C"))
              (for _array_element _outactors
                (bind _asbp_enemy_cone (Utilities|Casting|CastTobp_enemy_cone _array_element))
                (Default|ChooseTile _asbp_enemy_cone)
                (Development|PrintString "Hello"))))
          (elif (Math|Float|NearlyEqual(Float) (Variables|/Game/Blueprints/controllers/bp_ctlr_rhythm.bp_ctlr_rhythm_C|GetrhythmValue (Variables|Default|GetrhythmControllerRef)) 1.0 0.01)
            (switch Utilities|FlowControl|Switch|Switchone_rhythmState (Variables|/Game/Blueprints/controllers/bp_ctlr_rhythm.bp_ctlr_rhythm_C|GetrhythmState (Variables|Default|GetrhythmControllerRef))
              (:NewEnumerator1
                (bind _outactors_2 (Actor|GetAllActorsOfClass "/Game/Blueprints/enemies/bp_enemy_cube.bp_enemy_cube_C"))
                (for _array_element_2 _outactors_2
                  (bind _asbp_enemy_cube (Utilities|Casting|CastTobp_enemy_cube _array_element_2))
                  (Default|CubeAttack _asbp_enemy_cube))))))))))

(fn ConstructionScript)

(fn SpawnEnemyatLocation
  (params (enemyToSpawn :type Bp%20Enemy%20Parent%20Class%20Reference) (X :type Integer) (Y :type Integer) (enemyType :type e_enemyTypes%20Enum :default "NewEnumerator0") (randomize? :type Boolean))
  (bind _playercontrollerref (Variables|Default|GetplayerControllerRef))
  (bind _playercontrollerref_2 (Variables|Default|GetplayerControllerRef))
  (if randomize?
    (Utilities|FlowControl|Sequence
      (:then_0
        ;[1 1 1] set local vars
        (LocalVariables|SetX1 (Math|Random|RandomIntegerinRange 0 (- (Variables|/Game/Blueprints/controllers/bp_ctlr_player.bp_ctlr_player_C|GetgridHorizontal _playercontrollerref) 1)) :!label _label)
        (LocalVariables|SetY1 (Math|Random|RandomIntegerinRange 0 (- (Variables|/Game/Blueprints/controllers/bp_ctlr_player.bp_ctlr_player_C|GetgridVertical _playercontrollerref) 1)))
        (LocalVariables|SetenemyClass enemyToSpawn)
        (LocalVariables|SetlocalEnemyType enemyType))
      (:then_1
        ;[1 1 1] get grid square at XY
        (bind _element (Utilities|Get2dArray (Variables|/Game/Blueprints/controllers/bp_ctlr_player.bp_ctlr_player_C|GetgridArray _playercontrollerref_2) (LocalVariables|GetX1) (LocalVariables|GetY1) (Variables|/Game/Blueprints/controllers/bp_ctlr_player.bp_ctlr_player_C|GetgridHorizontal _playercontrollerref_2) :!label _label_2)
          (:1
            (if (Variables|/Game/Blueprints/bp_gridSquare.bp_gridSquare_C|Getimpassable? _element)
              _
              (else
                (Utilities|IsValid (Variables|/Game/Blueprints/bp_gridSquare.bp_gridSquare_C|GetactorHere _element)
                  (:Is%20Valid
                    _)
                  (:Is%20Not%20Valid
                    ;[1 1 1] if no enemy actor at XY location, spawn enemy
                    (bind _returnvalue (Game|SpawnActorfromClass (LocalVariables|GetenemyClass) (Math|Transform|MakeTransform (Math|Vector|MakeVector (.x (Transformation|GetActorLocation _element)) (.y (Transformation|GetActorLocation _element)) (+ (.z (Transformation|GetActorLocation _element)) 1e+02)) "0, 0, 0" "1,1,1") "Undefined" 0 (Variables|Default|GetplayerControllerRef) (Variables|Default|GetrhythmControllerRef) self (Utilities|Select :Index (LocalVariables|GetlocalEnemyType) :NewEnumerator0 "NewEnumerator0" :NewEnumerator1 "NewEnumerator1" :NewEnumerator2 "NewEnumerator2") (Math|Vector|MakeVector (Math|Conversions|ToFloat(Integer) (LocalVariables|GetX1)) (Math|Conversions|ToFloat(Integer) (LocalVariables|GetY1)) 0.0) 0 0))
                    ;[1 1 1] add enemy to enemy array
                    (Utilities|Array|Add (Variables|Default|GetenemyArray) _returnvalue)
                    ;[1 1 1] update grid square
                    (Variables|/Game/Blueprints/bp_gridSquare.bp_gridSquare_C|SetactorHere _element _returnvalue)
                    ;[1 1 1] add to individual enemy type array
                    (if (== (LocalVariables|GetenemyClass) "/Game/Blueprints/enemies/bp_enemy_cone.bp_enemy_cone_C")
                      (Utilities|Array|Add (Variables|Default|GetenemyConeArray) _returnvalue)
                      (return)
                      (elif (== (LocalVariables|GetenemyClass) "/Game/Blueprints/enemies/bp_enemy_cube.bp_enemy_cube_C")
                        (Utilities|Array|Add (Variables|Default|GetenemyCubeArray) _returnvalue)
                        (return)
                        (elif (== (LocalVariables|GetenemyClass) "/Game/Blueprints/enemies/bp_enemy_cylinder.bp_enemy_cylinder_C")
                          (Utilities|Array|Add (Variables|Default|GetenemyCylinderArray) _returnvalue)
                          (return)
                          (else
                            (return)))))))))
            (CallFunction|SpawnEnemyatLocation (LocalVariables|GetenemyClass) 0 0 (LocalVariables|GetlocalEnemyType) true)))))
    (else
      (Utilities|FlowControl|Sequence
        (:then_0
          (goto _label))
        (:then_1
          (goto _label_2))))))

(fn DestroyAllEnemies
  (for _array_element (Variables|Default|GetenemyArray)
    (Actor|DestroyActor _array_element)))
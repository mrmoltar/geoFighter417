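; Poison pickup that poisons the player when picked up, passing its poison length and damage to the player and printing a debug message.
; On BeginPlay it registers itself in the enemy controller's poison pickup array, reached through the player controller, before calling the parent.
; Its decrementLife event counts down PoisonDecay until the pickup expires.
; Both expiry and pickup remove it from its stored array and destroy the actor.
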(event Custom|decrementLife
  (bind _poisondecay (Variables|Default|GetpoisonDecay))
  (if (> _poisondecay 1)
    (Math|Integer|DecrementInt _poisondecay)
    (else
      (CallFunction|DestorySelf))))

(event EventBeginPlay
  (bind _playercontrollerref (Variables|Default|GetplayerControllerRef))
  (bind _enemycontrollerref (Variables|/Game/Blueprints/controllers/bp_ctlr_player.bp_ctlr_player_C|GetenemyControllerRef _playercontrollerref))
  (bind _poisonpickuparray (Variables|/Game/Blueprints/controllers/bp_ctlr_enemy.bp_ctlr_enemy_C|GetpoisonPickupArray _enemycontrollerref))
  (Variables|Default|SetpickupArray _poisonpickuparray)
  (Utilities|Array|Add _poisonpickuparray self)
  (|CallParentFunction))

(event Collision|EventActorBeginOverlap
  (params (OtherActor :type Actor%20Object%20Reference))
  (|CallParentFunction OtherActor))

(event EventTick
  (params (DeltaSeconds :type Float%20%28single-precision%29))
  (|CallParentFunction DeltaSeconds))

(event EventPickup
  (bind _playercontrollerref (Variables|Default|GetplayerControllerRef))
  (bind _playerref (Variables|/Game/Blueprints/controllers/bp_ctlr_player.bp_ctlr_player_C|GetplayerRef _playercontrollerref))
  (Variables|/Game/Blueprints/bp_player.bp_player_C|Setpoisoned? _playerref true)
  (Variables|/Game/Blueprints/bp_player.bp_player_C|SetpoisonLength _playerref (Variables|Default|GetpoisonLength))
  (Variables|/Game/Blueprints/bp_player.bp_player_C|SetpoisonDamage _playerref (Variables|Default|GetpoisonDamage))
  (Development|PrintString "PLAYER POISONED" true true "(R=0.180740,G=1.000000,B=0.000000,A=1.000000)" 4.0)
  (CallFunction|DestorySelf))

(fn ConstructionScript
  (|CallParentFunction))

(fn DestorySelf
  (Utilities|Array|RemoveItem (Variables|Default|GetpickupArray) self)
  (Actor|DestroyActor))
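; Experience pickup Blueprint that grants the player Exp when collected.
; Its Pickup event adds ExpToAdd to the player's Exp through the PlayerController reference, tells the music controller to play its ExpPickup response, then destroys itself.
; BeginPlay, overlap and Tick are unused stubs, so collection is triggered from outside this graph.
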(event EventBeginPlay
  (|CallParentFunction))

(event Collision|EventActorBeginOverlap
  (params (OtherActor :type Actor%20Object%20Reference))
  (|CallParentFunction OtherActor))

(event EventTick
  (params (DeltaSeconds :type Float%20%28single-precision%29))
  (|CallParentFunction DeltaSeconds))

(event EventPickup
  (bind _playercontrollerref (Variables|Default|GetplayerControllerRef))
  (bind _playerref (Variables|/Game/Blueprints/controllers/bp_ctlr_player.bp_ctlr_player_C|GetplayerRef _playercontrollerref))
  (Variables|/Game/Blueprints/bp_player.bp_player_C|Setexp _playerref (+ (Variables|/Game/Blueprints/bp_player.bp_player_C|Getexp _playerref) (Variables|Default|GetexpToAdd)))
  (Default|ExpPickup (Variables|/Game/Blueprints/controllers/bp_ctlr_player.bp_ctlr_player_C|GetmusicControllerRef (Variables|Default|GetplayerControllerRef)))
  (Actor|DestroyActor))

(fn ConstructionScript
  (|CallParentFunction))
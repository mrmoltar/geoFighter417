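; Base enemy actor for cone, cube and cylinder types, with random spin and links to the player and rhythm controllers.
; TakeDamage destroys the enemy on lethal damage, otherwise plays a sound and sets Health to damage minus Health (operands reversed from usual subtraction).
; DestroySelf clears its tile, notifies the music controller of the death by type, and removes itself from the enemy controller's arrays before destroying the actor.
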(event EventBeginPlay
  (Variables|/Script/Engine.RotatingMovementComponent|SetRotationRate (Variables|Default|GetRotatingMovement) (Math|Rotator|MakeRotator (Math|Random|RandomFloatinRange 15.0 1.2e+02) (Math|Random|RandomFloatinRange 15.0 1.2e+02) 9e+01))
  (bind _asbp_ctlr_player (Utilities|Casting|CastTobp_ctlr_player (Game|GetPlayerController 0)))
  (bind _output_get (Variables|Refs|SetplayerControllerRef _asbp_ctlr_player))
  (Variables|Refs|SetrhythmControllerRef (Variables|/Game/Blueprints/controllers/bp_ctlr_player.bp_ctlr_player_C|GetrhythmControllerRef _output_get)))

(event Collision|EventActorBeginOverlap
  (params (OtherActor :type Actor%20Object%20Reference)))

(fn ConstructionScript)

(fn TakeDamage
  (params (damageToTake :type Integer))
  (if (>= damageToTake (Variables|Default|Gethealth))
    (CallFunction|DestroySelf)
    (else
      (Audio|SpawnSound2D "/Engine/EditorSounds/Notifications/CompileFailed.CompileFailed" 0.2)
      (Variables|Default|Sethealth (- damageToTake (Variables|Default|Gethealth)))))
  (return))

(fn DestroySelf
  (bind _enemycontrollerref (Variables|refs|GetenemyControllerRef))
  (bind _enemytype (Variables|Default|GetenemyType))
  (bind _enemycontrollerref_2 (Variables|refs|GetenemyControllerRef))
  (bind _enemyconearray (Variables|/Game/Blueprints/controllers/bp_ctlr_enemy.bp_ctlr_enemy_C|GetenemyConeArray _enemycontrollerref))
  (bind _enemycubearray (Variables|/Game/Blueprints/controllers/bp_ctlr_enemy.bp_ctlr_enemy_C|GetenemyCubeArray _enemycontrollerref))
  (bind _enemycylinderarray (Variables|/Game/Blueprints/controllers/bp_ctlr_enemy.bp_ctlr_enemy_C|GetenemyCylinderArray _enemycontrollerref))
  (bind _enemyarray (Variables|/Game/Blueprints/controllers/bp_ctlr_enemy.bp_ctlr_enemy_C|GetenemyArray _enemycontrollerref_2))
  (bind _returnvalue (Utilities|Select :Index _enemytype :NewEnumerator0 _enemyconearray :NewEnumerator1 _enemycubearray :NewEnumerator2 _enemycylinderarray))
  (Variables|/Game/Blueprints/bp_gridSquare.bp_gridSquare_C|SetactorHere (Variables|Default|GetcurrentTile) 0)
  (Default|EnemyDeath (Variables|/Game/Blueprints/controllers/bp_ctlr_player.bp_ctlr_player_C|GetmusicControllerRef (Variables|Refs|GetplayerControllerRef)) (Variables|Default|GetenemyType))
  (for _array_element _returnvalue
    (if (== _array_element self)
      (Utilities|Array|RemoveItem _returnvalue _array_element)))
  (for _array_element_2 _enemyarray
    (if (== _array_element_2 self)
      (Utilities|Array|RemoveItem _enemyarray _array_element_2)))
  (Actor|DestroyActor)
  (return))
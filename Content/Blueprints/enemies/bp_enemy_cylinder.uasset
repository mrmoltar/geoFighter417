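; Cylinder enemy for a tile-grid game that steps to the neighbouring tile farthest from the player.
; When chooseTileCylinder fires and its Player variable is invalid, GetChosenTile scores free, passable surrounding tiles by Manhattan distance to the player.
; MoveActor snaps the enemy to the highest-scoring tile, updates coordinates and tile occupancy, then the neighbours are refreshed.
; A separate cylinderMove event only updates tile occupancy and clears the neighbour list.
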(event Custom|chooseTileCylinder
  (bind _currentcoords (Variables|Default|GetcurrentCoords))
  (Utilities|IsValid (Variables|Default|Getplayer)
    (:Is%20Not%20Valid
      (bind (_lowesthgrid1 _highesthgrid1 _heuristicarray1) (CallFunction|GetChosenTile (Variables|Default|GetsurroundingTiles) false true))
      (Variables|Default|SetselectedGridTile _highesthgrid1)
      (Variables|Default|SethArray _heuristicarray1)
      (Utilities|IsValid (Variables|/Game/Blueprints/bp_gridSquare.bp_gridSquare_C|GetactorHere _highesthgrid1)
        (:Is%20Not%20Valid
          (Utilities|IsValid (Variables|Default|Getplayer)
            (:Is%20Not%20Valid
              (if (not (Variables|/Game/Blueprints/bp_gridSquare.bp_gridSquare_C|Getimpassable? _highesthgrid1))
                (Variables|Default|SetChosenTile _highesthgrid1)
                (CallFunction|MoveActor (Variables|Default|GetChosenTile))
                (bind _surroundingtiles (CallFunction|GetSurroundingTiles 1 (Math|Float|Truncate (.x _currentcoords)) (Math|Float|Truncate (.y _currentcoords))))
                (Variables|Default|SetsurroundingTiles _surroundingtiles)))))))))

(event Custom|cylinderMove
  (Utilities|IsValid (Variables|Default|GetpreviousGridSquare)
    (:Is%20Valid
      (if (== (Variables|Default|GetpreviousGridSquare) (Variables|Default|GetcurrentTile))
        _
        (else
          (Variables|Default|SetpreviousGridSquare (Variables|Default|GetcurrentTile) :!label _label))))
    (:Is%20Not%20Valid
      (goto _label)))
  (Variables|/Game/Blueprints/bp_gridSquare.bp_gridSquare_C|SetactorHere (Variables|Default|GetpreviousGridSquare) 0)
  (Variables|Default|SetcurrentTile (Variables|Default|GetChosenTile))
  (Variables|/Game/Blueprints/bp_gridSquare.bp_gridSquare_C|SetactorHere (Variables|Default|GetcurrentTile) self)
  (Utilities|Array|Clear (Variables|Default|GetsurroundingTiles)))

(event EventBeginPlay
  (bind _currentcoords (Variables|Default|GetcurrentCoords))
  (bind _surroundingtiles (CallFunction|GetSurroundingTiles 1 (Math|Float|Truncate (.x _currentcoords)) (Math|Float|Truncate (.y _currentcoords))))
  (Variables|Default|SetsurroundingTiles _surroundingtiles))

(fn ConstructionScript
  (|CallParentFunction))

(fn GetChosenTile
  (params (grid :type Array%20of%20Bp%20Grid%20Square%20Object%20References) (findLowest? :type Boolean) (ignoreImpassableTiles? :type Boolean))
  (bind _multiplelowesth (LocalVariables|GetmultipleLowestH))
  (bind _multiplehighesth (LocalVariables|GetmultipleHighestH))
  (bind _returnvalue (Utilities|Array|Length _multiplehighesth))
  (bind _returnvalue_2 (Utilities|Array|Length _multiplelowesth))
  (LocalVariables|SetI ignoreImpassableTiles?)
  (LocalVariables|SetL findLowest?)
  (bind _output_get (LocalVariables|SetlocalGridArray grid))
  (for _array_element _output_get
    (if (LocalVariables|GetI)
      (Utilities|IsValid (Variables|/Game/Blueprints/bp_gridSquare.bp_gridSquare_C|GetactorHere _array_element)
        (:Is%20Not%20Valid
          (if (not (Variables|/Game/Blueprints/bp_gridSquare.bp_gridSquare_C|Getimpassable? _array_element))
            (Utilities|Map|Add (LocalVariables|GetheuristicArray) _array_element (Math|Float|Truncate (+ (Math|Float|Absolute(Float) (.x (- (Variables|/Game/Blueprints/bp_player.bp_player_C|GetcurrentCoords (Variables|/Game/Blueprints/controllers/bp_ctlr_player.bp_ctlr_player_C|GetplayerRef (Variables|Default|GetplayerControllerRef))) (Variables|/Game/Blueprints/bp_gridSquare.bp_gridSquare_C|GetcurrentCoords _array_element)))) (Math|Float|Absolute(Float) (.y (- (Variables|/Game/Blueprints/bp_player.bp_player_C|GetcurrentCoords (Variables|/Game/Blueprints/controllers/bp_ctlr_player.bp_ctlr_player_C|GetplayerRef (Variables|Default|GetplayerControllerRef))) (Variables|/Game/Blueprints/bp_gridSquare.bp_gridSquare_C|GetcurrentCoords _array_element)))))) :!label _label))))
      (else
        (goto _label))))
  (bind _keys (Utilities|Map|Keys (LocalVariables|GetheuristicArray)))
  (for (_array_element_2 _array_index) _keys
    (LocalVariables|SethElement (.Value (Utilities|Map|Find (LocalVariables|GetheuristicArray) _array_element_2)))
    (LocalVariables|SethIndex _array_index)
    (LocalVariables|SethActor _array_element_2)
    (if (LocalVariables|GetL)
      ;[1 1 1] is less than lowest h
      (if (< (LocalVariables|GethElement) (LocalVariables|GetlowestH))
        (Utilities|Map|Add (LocalVariables|GetheuristicArray) (LocalVariables|GethActor) (LocalVariables|GethElement))
        (LocalVariables|SetlowestHGrid (LocalVariables|GethActor))
        (LocalVariables|SetlowestH (LocalVariables|GethElement)))
      (else
        ;[1 1 1] is greater than highest h
        (if (> (LocalVariables|GethElement) (LocalVariables|GethightestH))
          (Utilities|Map|Add (LocalVariables|GetheuristicArray) (LocalVariables|GethActor) (LocalVariables|GethElement))
          (LocalVariables|SethighestHGrid (LocalVariables|GethActor))
          (LocalVariables|SethightestH (LocalVariables|GethElement))))))
  (Utilities|FlowControl|Sequence
    (:then_0
      (if (> _returnvalue_2 1)
        (LocalVariables|SetlowestHGrid (Utilities|Array|Get(acopy) (LocalVariables|GetlocalGridArray) (Math|Random|RandomInteger _returnvalue_2)))))
    (:then_1
      (if (> _returnvalue 1)
        (LocalVariables|SethighestHGrid (Utilities|Array|Get(acopy) (LocalVariables|GetlocalGridArray) (Math|Random|RandomInteger _returnvalue)))))
    (:then_2
      (return (LocalVariables|GetlowestHGrid) (LocalVariables|GethighestHGrid) (LocalVariables|GetheuristicArray)))))

(fn MoveActor
  (params (otherActor :type Actor%20Object%20Reference))
  (bind _returnvalue (Transformation|GetActorLocation otherActor))
  (Variables|Default|SetpreviousGridSquare (Variables|Default|GetcurrentTile))
  (bind _asbp_grid_square (Utilities|Casting|CastTobp_gridSquare otherActor))
  (Variables|Default|SetcurrentTile _asbp_grid_square)
  ;[1 1 1] move to new location
  (Transformation|SetWorldLocation (Variables|Transformation|GetRootComponent) (Math|Vector|MakeVector (.x _returnvalue) (.y _returnvalue) (Variables|Default|GetzOffset)) false false)
  (Variables|Default|SetcurrentCoords (Variables|/Game/Blueprints/bp_gridSquare.bp_gridSquare_C|GetcurrentCoords (Variables|Default|GetcurrentTile)))
  (Variables|/Game/Blueprints/bp_gridSquare.bp_gridSquare_C|SetactorHere (Variables|Default|GetcurrentTile) self)
  (Variables|/Game/Blueprints/bp_gridSquare.bp_gridSquare_C|SetactorHere (Variables|Default|GetpreviousGridSquare) 0))
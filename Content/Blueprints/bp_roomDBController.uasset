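; Room database controller that decodes image-based room layouts, where pixel colours stand for floors, walls, doors, traps and enemies.
; BeginPlay counts the room images and builds an ordered colour array, whose matching index converts a colour into a feature/enemy enum.
; A helper fetches a room's pixels by image index from the Bp_roomDB_obj actor.
; The pass that re-sorts rooms by door layout and updates that actor is disconnected.
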(event EventBeginPlay
  (bind _roomimagenumber (CallFunction|GetRoomImageTotal))
  (Variables|COLORCODES|SetcolorCodesArray (Utilities|Array|MakeArray (Variables|COLORCODES|Getfloor_color) (Variables|COLORCODES|Getwall_color) (Variables|COLORCODES|Getdoor_Color) (Variables|COLORCODES|GetspringBoardN_color) (Variables|COLORCODES|GetspringBoardNE_color) (Variables|COLORCODES|GetspringBoardE_color) (Variables|COLORCODES|GetspringBoardSE_color) (Variables|COLORCODES|GetspringBoardS_color) (Variables|COLORCODES|GetspringBoardSW_color) (Variables|COLORCODES|GetspringBoardW_color) (Variables|COLORCODES|GetspringBoardNW_color) (Variables|COLORCODES|GetbombLauncherN_color) (Variables|COLORCODES|GetbombLauncherNE_color) (Variables|COLORCODES|GetbombLauncherE_color) (Variables|COLORCODES|GetbombLauncherSE_color) (Variables|COLORCODES|GetbombLauncherS_color) (Variables|COLORCODES|GetbombLauncherSW_color) (Variables|COLORCODES|GetbombLauncherW_color) (Variables|COLORCODES|GetbombLauncherNW_color) (Variables|COLORCODES|Getspike_color) (Variables|COLORCODES|Getpit_color) (Variables|COLORCODES|Getenemy_stationary_color) (Variables|COLORCODES|Getenemy_pursuer_color) (Variables|COLORCODES|Getenemy_runner_color))))

(fn ConstructionScript)

(fn ClearAllDoorArrays
  (Utilities|Array|Clear (Variables|DEFAULTDOORS|GetnorthDoors))
  (Utilities|Array|Clear (Variables|DEFAULTDOORS|GeteastDoors))
  (Utilities|Array|Clear (Variables|DEFAULTDOORS|GetsouthDoors))
  (Utilities|Array|Clear (Variables|DEFAULTDOORS|GetsouthDoors))
  (Utilities|Array|Clear (Variables|DEFAULTDOORS|GetwestDoors))
  (Utilities|Array|Clear (Variables|DEFAULTDOORS|GetnorthEastDoors))
  (Utilities|Array|Clear (Variables|DEFAULTDOORS|GetnorthEastSouthDoors))
  (Utilities|Array|Clear (Variables|DEFAULTDOORS|GetnorthEastSouthWestDoors))
  (Utilities|Array|Clear (Variables|DEFAULTDOORS|GeteastSouthDoors))
  (Utilities|Array|Clear (Variables|DEFAULTDOORS|GeteastSouthWestDoors))
  (Utilities|Array|Clear (Variables|DEFAULTDOORS|GetsouthWestDoors))
  (Utilities|Array|Clear (Variables|DEFAULTDOORS|GetnorthSouthDoors))
  (Utilities|Array|Clear (Variables|DEFAULTDOORS|GeteastWestDoors))
  (Utilities|Array|Clear (Variables|DEFAULTDOORS|GetnorthWestEastDoors))
  (Utilities|Array|Clear (Variables|DEFAULTDOORS|GetnorthWestSouthDoors))
  (Utilities|Array|Clear (Variables|DEFAULTDOORS|GetnorthWestDoors)))

(fn GetFeature/EnemyfromColor
  (params (color :type Linear%20Color%20Structure))
  (bind (_r _g _b) (Math|Color|BreakColor color))
  (for (_array_element _array_index) (Variables|COLORCODES|GetcolorCodesArray)
    (if (Math|Vector|Equal(Vector) _array_element (Math|Vector|MakeVector _r _g _b) 0.0001)
      (bind _output_get (LocalVariables|SetenemyOrFeature (Utilities|Enum|ByteToEnume_enemiesAndFeatures (Math|Conversions|ToByte(Integer) _array_index))))
      (return true _output_get _array_element _array_index)))
  (return false "NewEnumerator1" "0, 0, 0" 0))

(fn GetRoomImageTotal
  (bind _roomimagenumber (Variables|Default|GetroomImageNumber))
  (for _array_element (Variables|Default|GetroomDB)
    (Math|Integer|IncrementInt _roomimagenumber))
  (return _roomimagenumber))

(fn FindImageIndexinRoomArrays
  (params (indexToFind :type Integer))
  (bind _outactors (Actor|GetAllActorsOfClass "/Game/Blueprints/bp_roomDB_obj.bp_roomDB_obj_C"))
  (for _array_element (Variables|/Game/Blueprints/bp_roomDB_obj.bp_roomDB_obj_C|Getdb_new (Utilities|Array|Get(acopy) _outactors))
    (if (== (.roomImageIndex (Utilities|Struct|Breakstruct_room_pixelsAndDoors _array_element)) indexToFind)
      (return (.pixels (Utilities|Struct|Breakstruct_room_pixelsAndDoors _array_element))))))